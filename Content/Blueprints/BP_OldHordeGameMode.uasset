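; Game mode for Old Horde, a Mordhau wave-survival mode that also tracks player kills and handles purchased team revives.
; BeginPlay loads server config options, removes kill-objective nobles and caches horde spawn points.
; SpawnWave picks a random wave variant and spawns enemies up to an alive cap, using pooled AI controllers and database-driven classes, gear and customization.
; OnKilled recycles the dead bot's controller to spawn replacements from the variant's remaining counts.
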(event `self.ReceiveBeginPlay`
  (bind _isvalid (`self.GetConfig`))
  (if (not _isvalid)
    (`MordhauUtilityLibrary.PrintToConsoleAndLog` "[DEBUG] Config Load Failed"))
  (`self.KillNobles`)
  (`parent.ReceiveBeginPlay`)
  (bind _outactors (`GameplayStatics.GetAllActorsOfClass` "/Game/Mordhau/Blueprints/GameModes/Horde/BP_HordeSpawn.BP_HordeSpawn_C"))
  (set `self.HordeSpawns` _outactors)
  (`|ExecutionSequence`
    (:`then_0`
      (if (`self.TeamDamage`)
        (set `self.TeamDamageFactor` 0.5)
        (else
          (set `self.TeamDamageFactor` 0.0))))
    (:`then_1`
      (if (`self.EnableSkillTree`)
        (bind _asbp_old_horde_game_state (cast `/OldHorde/Blueprints/BP_OldHordeGameState` (`GameplayStatics.GetGameState`)))
        (set `/OldHorde/Blueprints/BP_OldHordeGameState.UseSkillTree` true _asbp_old_horde_game_state)))))

(event `self.OnKilled`
  (params (Killer :type "Controller Object Reference") (KilledPlayer :type "Controller Object Reference") (KilledPawn :type "Pawn Object Reference") (Type :type "EMordhauDamageType Enum" :default "Generic") (SubType :type Byte) (DamageSource :type "Actor Object Reference") (DamageAgent :type "Actor Object Reference"))
  (`parent.OnKilled` Killer KilledPlayer KilledPawn Type SubType DamageSource DamageAgent)
  (`|ExecutionSequence`
    (:`then_0`
      (if (< (`KismetArrayLibrary.Array_Length` (`self.SpawnedEnemies`)) (`self.WaveMax`))
        (if (> (`BlueprintMapLibrary.Map_Length` (`.Enemies_4_C909441D45A9BD4354B2C59324F03101` (break `/Game/Mordhau/Blueprints/GameModes/Horde/STRUCT_HordeEnemyArray` (`self.CurrentWaveVariant`)))) 0)
          (bind _asbp_horde_aicontroller (cast `/Game/Mordhau/AI/BP_HordeAIController` (`AIBlueprintHelperLibrary.GetAIController` KilledPawn)))
          (`/Engine/EditorBlueprintResources/StandardMacros.DecrementInt` (`self.TotalAlive`)
            (:`  `
              (if (> (`BlueprintMapLibrary.Map_Length` (`.Enemies_4_C909441D45A9BD4354B2C59324F03101` (break `/Game/Mordhau/Blueprints/GameModes/Horde/STRUCT_HordeEnemyArray` (`self.CurrentWaveVariant`)))) 0)
                (bind _enemyname (`self.GetEnemyToRespawn`))
                (if (not (== _enemyname "None"))
                  (`self.SpawnEnemy` _enemyname _asbp_horde_aicontroller))))))))
    (:`then_1`
      (bind _asbp_old_horde_player_controller (cast `/OldHorde/Blueprints/BP_OldHordePlayerController` Killer))
      (set `/OldHorde/Blueprints/BP_OldHordePlayerController.KillCounter` (+ (`/OldHorde/Blueprints/BP_OldHordePlayerController.KillCounter` _asbp_old_horde_player_controller) 1) _asbp_old_horde_player_controller))))

(event `HealTeamOnServer`
  (for _array_element (`self.ReviveControllers`)
    (`self.RestartPlayer` _array_element))
  (`/Engine/EditorBlueprintResources/ActorMacros.Switch Has Authority`
    (:`Authority`
      (bind _outactors (`GameplayStatics.GetAllActorsOfClass` "/Game/Mordhau/Blueprints/Characters/BP_HordeCharacter.BP_HordeCharacter_C"))
      (for _array_element_2 _outactors
        (if (not (`AdvancedCharacter.GetIsDead` _array_element_2))
          (`AdvancedCharacter.OffsetHealth` _array_element_2 100 true))))))

(event `HealTeam`
  (params (Character :type "/Game/Mordhau/Blueprints/Characters/BP_HordeCharacter Object Reference"))
  (bind _returnvalue (`AdvancedCharacter.GetControllerIncludingVehicle` Character))
  (bind _outactors (`GameplayStatics.GetAllActorsOfClass` "/OldHorde/Blueprints/BP_OldHordePlayerController.BP_OldHordePlayerController_C"))
  (if (> (`KismetArrayLibrary.Array_Length` _outactors) 0)
    (for _array_element _outactors
      (bind _returnvalue_2 (`MordhauPlayerController.GetControlledMordhauCharacter` _array_element true))
      (`/Engine/EditorBlueprintResources/StandardMacros.IsValid` _returnvalue_2
        (:`Is Valid`
          (if (`AdvancedCharacter.GetIsDead` _returnvalue_2)
            (`self.RestartPlayer` _array_element :!label _label)
            (set `/OldHorde/Blueprints/BP_OldHordePlayerController.ReviveCounter` (+ (`/OldHorde/Blueprints/BP_OldHordePlayerController.ReviveCounter` _array_element) 1) _array_element)))
        (:`Is Not Valid`
          (goto _label))))
    (`self.Broadcast` self (`KismetStringLibrary.Concat_StrStr` (`PlayerState.GetPlayerName` (`Controller.PlayerState` _returnvalue)) " has purchased a Team Revive!") "ServerSay")
    (bind _asbp_old_horde_player_controller (cast `/OldHorde/Blueprints/BP_OldHordePlayerController` _returnvalue))
    (set `/OldHorde/Blueprints/BP_OldHordePlayerController.ReviveCounter` (+ (`/OldHorde/Blueprints/BP_OldHordePlayerController.ReviveCounter` _asbp_old_horde_player_controller) 1) _asbp_old_horde_player_controller)))

(fn `AttachComponentsToEnemy`
  (params (HordeAIController :type "/Game/Mordhau/AI/BP_HordeAIController Object Reference") (CustomizationReplicationActor :type "CustomizationReplicationActor Object Reference") (Equips1 :type "Array of MordhauEquipment Class Reference (by ref)") (Equips2 :type "Array of MordhauEquipment Class Reference (by ref)") (Enemy :type "/Game/Mordhau/Blueprints/GameModes/Horde/BP_HordeEnemy Object Reference (by ref)"))
  (set `AdvancedCharacter.Team` 1 Enemy)
  (`MordhauCharacter.SetCustomizationReplicationActor` Enemy CustomizationReplicationActor)
  (`Controller.Possess` HordeAIController Enemy)
  (`self.SpawnEquipmentFor` Equips1 Enemy)
  (`self.SpawnEquipmentFor` Equips2 Enemy)
  (`MordhauCharacter.OnPostProfileAssigned` Enemy))

(fn `GetConfig`
  (returns (IsValid :type Boolean))
  (bind (_isvalid _returnvalue) (`MordhauUtilityLibrary.GetCustomConfigVar_Float` "OldHorde" "TimeBetweenWaves"))
  (bind (_isvalid_2 _returnvalue_2) (`MordhauUtilityLibrary.GetCustomConfigVar_Bool` "OldHorde" "EnableSkillTree"))
  (bind (_isvalid_3 _returnvalue_3) (`MordhauUtilityLibrary.GetCustomConfigVar_Int` "OldHorde" "MaxEnemiesAlive"))
  (bind (_isvalid_4 _returnvalue_4) (`MordhauUtilityLibrary.GetCustomConfigVar_Bool` "OldHorde" "EnableTeamDamage"))
  (bind (_isvalid_5 _returnvalue_5) (`MordhauUtilityLibrary.GetCustomConfigVar_Bool` "OldHorde" "EnableSell"))
  (bind (_isvalid_6 _returnvalue_6) (`MordhauUtilityLibrary.GetCustomConfigVar_Bool` "OldHorde" "EnableExplosives"))
  (`/Engine/EditorBlueprintResources/ActorMacros.Switch Has Authority`
    (:`Authority`
      (`|ExecutionSequence`
        (:`then_0`
          (if _isvalid_3
            (set `self.MaxAliveEnemies` _returnvalue_3)))
        (:`then_1`
          (if _isvalid_4
            (set `self.TeamDamage` _returnvalue_4)))
        (:`then_2`
          (if _isvalid
            (set `self.WaveEnemySpawnOffset` _returnvalue)))
        (:`then_3`
          (if (and _isvalid_5 _returnvalue_5)
            (set `self.EnableSell` true)
            (else
              (set `self.EnableSell` false))))
        (:`then_4`
          (if (and _isvalid_6 _returnvalue_6)
            (set `self.EnableExplosives` true)
            (else
              (set `self.EnableExplosives` false))))
        (:`then_5`
          (if (and _isvalid_2 _returnvalue_2)
            (set `self.EnableSkillTree` true)))
        (:`then_6`
          (return true))))))

(fn `GetCustomizationEnemy`
  (params (EnemyName :type Name))
  (returns (HordeEnemyClsRef :type "/Game/Mordhau/Blueprints/GameModes/Horde/BP_HordeEnemy Class Reference") (EquipmentArray :type "Array of MordhauEquipment Class Reference") (SecondaryEquipmentArray :type "Array of MordhauEquipment Class Reference") (BotBehaviourClsREf :type "BotBehaviorProfile Class Reference") (EnemyVariantCustomizationActor :type "Actor Object Reference"))
  (bind (_charactertype _customizationvariants _equipment _secondaryequipment _behavior) (break `/Game/Mordhau/Blueprints/GameModes/Horde/STRUCT_HordeEnemyInfo` (`BlueprintMapLibrary.Map_Find` (`self.EnemyDatabase`) EnemyName)))
  (bind _actors (break `ArrayOfActor` (`BlueprintMapLibrary.Map_Find` (`self.EnemyVariantCustomizationActor`) EnemyName)))
  (return _charactertype _equipment _secondaryequipment _behavior (`|GetArrayItem` _actors (`KismetMathLibrary.RandomInteger` (`KismetArrayLibrary.Array_Length` _actors)))))

(fn `GetEnemyToRespawn`
  (returns (EnemyName :type Name))
  (locals (TempName :type Name))
  (bind _tempname (`local.TempName`))
  (bind _enemies (break `/Game/Mordhau/Blueprints/GameModes/Horde/STRUCT_HordeEnemyArray` (`self.CurrentWaveVariant`)))
  (bind _value (`BlueprintMapLibrary.Map_Find` _enemies (`local.TempName`)))
  (bind _keys (`BlueprintMapLibrary.Map_Keys` (`.Enemies_4_C909441D45A9BD4354B2C59324F03101` (break `/Game/Mordhau/Blueprints/GameModes/Horde/STRUCT_HordeEnemyArray` (`self.CurrentWaveVariant`)))))
  (if (> (`KismetArrayLibrary.Array_Length` _keys) 0)
    (set `local.TempName` (`|GetArrayItem` _keys (`KismetMathLibrary.RandomInteger` (`BlueprintMapLibrary.Map_Length` _enemies))))
    (`BlueprintMapLibrary.Map_Add` (`.Enemies_4_C909441D45A9BD4354B2C59324F03101` (break `/Game/Mordhau/Blueprints/GameModes/Horde/STRUCT_HordeEnemyArray` (`self.CurrentWaveVariant`))) (`local.TempName`) (- _value 1))
    (if (not (> _value 0))
      (`BlueprintMapLibrary.Map_Remove` (`.Enemies_4_C909441D45A9BD4354B2C59324F03101` (break `/Game/Mordhau/Blueprints/GameModes/Horde/STRUCT_HordeEnemyArray` (`self.CurrentWaveVariant`))) _tempname))
    (return _tempname)
    (else
      (return "None"))))

(fn `KillNobles`
  (bind _outactors (`GameplayStatics.GetAllActorsOfClass` "/Game/Mordhau/Blueprints/GameModes/Horde/Objectives/BP_HordeKillObjective.BP_HordeKillObjective_C"))
  (if (> (`KismetArrayLibrary.Array_Length` _outactors) 0)
    (for _array_element _outactors
      (bind _returnvalue (`AdvancedCharacter.GetControllerIncludingVehicle` _array_element))
      (`/Engine/EditorBlueprintResources/StandardMacros.IsValid` _returnvalue
        (:`Is Valid`
          (`self.K2_DestroyActor` _returnvalue))
        (:`Is Not Valid`
          _))
      (`self.K2_DestroyActor` _array_element))))

(fn `OnRep_EnableExplosives`)

(fn `OnRep_EnableSell`)

(fn `OnRep_EnableSkillTree`
  (`self.SetSkillTree`))

(fn `OnRep_TeamDamage`)

(fn `PrepareAIControllers`
  (for _ (range (`self.MaxAliveEnemies`))
    (bind _returnvalue (`|SpawnActorFromClass` (`self.AIControllerClass`) (`KismetMathLibrary.MakeTransform` (0.0 0.0 0.0)) "Undefined" "OverrideRootScale" null null))
    (bind _asbp_horde_aicontroller (cast `/Game/Mordhau/AI/BP_HordeAIController` _returnvalue))
    (`KismetArrayLibrary.Array_Add` (`self.AIControllers`) _asbp_horde_aicontroller)))

(fn `ProgressWave`
  (`parent.ProgressWave`))

(fn `SetSkillTree`
  (if (`self.EnableSkillTree`)
    (bind _asbp_old_horde_game_state (cast `/OldHorde/Blueprints/BP_OldHordeGameState` (`GameplayStatics.GetGameState`)))
    (set `/OldHorde/Blueprints/BP_OldHordeGameState.UseSkillTree` true _asbp_old_horde_game_state)))

(fn `SetupCustomizationReplicationActors`
  (locals (Temp :type "Array of Actor Object Reference"))
  (bind _enemydatabase (`self.EnemyDatabase`))
  (bind _keys (`BlueprintMapLibrary.Map_Keys` _enemydatabase))
  (for _array_element _keys
    (`KismetArrayLibrary.Array_Clear` (`local.Temp`))
    (bind (_value _returnvalue) (`BlueprintMapLibrary.Map_Find` _enemydatabase _array_element))
    (if _returnvalue
      (for _array_element_2 (`.CustomizationVariants_23_31DB99B94B1F6227210491866A0F123E` (break `/Game/Mordhau/Blueprints/GameModes/Horde/STRUCT_HordeEnemyInfo` _value))
        (bind _returnvalue_2 (`|SpawnActorFromClass` "/Script/Mordhau.CustomizationReplicationActor" (`KismetMathLibrary.MakeTransform` (0.0 0.0 0.0)) "Undefined" "OverrideRootScale" null null))
        (`KismetArrayLibrary.Array_Add` (`local.Temp`) _returnvalue_2)
        (`CustomizationReplicationActor.AssignDataFromProfile` _returnvalue_2 _array_element_2))
      (`BlueprintMapLibrary.Map_Add` (`self.EnemyVariantCustomizationActor`) _array_element (make `ArrayOfActor` (`local.Temp`))))))

(fn `SpawnEnemy`
  (params (EnemyName :type Name) (`AI controller` :type "/Game/Mordhau/AI/BP_HordeAIController Object Reference (by ref)"))
  (locals (RandomChoice :type Integer) (EnemyToSpawn :type Name) (TempAIController :type "/Game/Mordhau/AI/BP_HordeAIController Object Reference"))
  (bind _returnvalue (`KismetMathLibrary.RandomInteger` 20))
  (bind _tempaicontroller (`local.TempAIController`))
  (bind _hordespawns (`self.HordeSpawns`))
  (bind (_charactertype _customizationvariants _equipment _secondaryequipment _behavior) (break `/Game/Mordhau/Blueprints/GameModes/Horde/STRUCT_HordeEnemyInfo` (`BlueprintMapLibrary.Map_Find` (`self.EnemyDatabase`) (`local.EnemyToSpawn`))))
  (bind _actors (break `ArrayOfActor` (`BlueprintMapLibrary.Map_Find` (`self.EnemyVariantCustomizationActor`) (`local.EnemyToSpawn`))))
  (set `local.EnemyToSpawn` EnemyName)
  (set `local.TempAIController` `AI controller`)
  (bind _returnvalue_2 (`|GenericCreateObject` _behavior _tempaicontroller))
  (set `MordhauAIController.BehaviorProfile` _returnvalue_2 _tempaicontroller)
  (bind _ascustomization_replication_actor (cast `CustomizationReplicationActor` (`|GetArrayItem` _actors (`KismetMathLibrary.RandomIntegerInRange` 0 (- (`KismetArrayLibrary.Array_Length` _actors) 1)))))
  (bind _output_get (set `MordhauAIController.CustomizationReplicationActor` _ascustomization_replication_actor _tempaicontroller))
  (bind _output_get_2 (set `local.RandomChoice` (`KismetMathLibrary.RandomInteger` (`KismetArrayLibrary.Array_Length` _hordespawns))))
  (bind _returnvalue_3 (`self.GetTransform` (`|GetArrayItem` _hordespawns _output_get_2)))
  (bind _returnvalue_4 (`|SpawnActorFromClass` _charactertype (`KismetMathLibrary.MakeTransform` (`KismetMathLibrary.TransformLocation` _returnvalue_3 (`KismetMathLibrary.MakeVector` (* (/ _returnvalue 6) 130.0) (* (mod _returnvalue 6) 130.0))) (.rotation _returnvalue_3)) "Undefined" "OverrideRootScale" null -1 null))
  (`KismetArrayLibrary.Array_Add` (`self.SpawnedEnemies`) _returnvalue_4)
  (set `AdvancedCharacter.Team` 1 _returnvalue_4)
  (`MordhauCharacter.SetCustomizationReplicationActor` _returnvalue_4 _output_get)
  (`Controller.Possess` (`local.TempAIController`) _returnvalue_4)
  (`self.SpawnEquipmentFor` _equipment _returnvalue_4)
  (`self.SpawnEquipmentFor` _secondaryequipment _returnvalue_4)
  (`MordhauCharacter.OnPostProfileAssigned` _returnvalue_4)
  (bind _asbp_horde_game_state (cast `/Game/Mordhau/Blueprints/GameModes/Horde/BP_HordeGameState` (`GameplayStatics.GetGameState`)))
  (bind (_wave _enemiesremaining _nextwavestarttime) (break `/Game/Mordhau/Blueprints/GameModes/Horde/STRUCT_HordeMatchInfo` (`/Game/Mordhau/Blueprints/GameModes/Horde/BP_HordeGameState.ReplicatedHordeMatchInfo` _asbp_horde_game_state)))
  (set `/Game/Mordhau/Blueprints/GameModes/Horde/BP_HordeGameState.ReplicatedHordeMatchInfo` (make `/Game/Mordhau/Blueprints/GameModes/Horde/STRUCT_HordeMatchInfo` _wave (`KismetMathLibrary.Conv_IntToByte` (`KismetMathLibrary.Clamp` (`self.WaveMax`) 0 255)) _nextwavestarttime (`KismetMathLibrary.Conv_IntToByte` (`KismetMathLibrary.Clamp` (`self.EnemiesSpawned`) 0 255))) _asbp_horde_game_state))

(fn `SpawnEnemyActor`
  (params (EnemyClass :type "/Game/Mordhau/Blueprints/GameModes/Horde/BP_HordeEnemy Class Reference") (NewParam1 :type "Array of Integer"))
  (returns (ReturnValue :type "/Game/Mordhau/Blueprints/GameModes/Horde/BP_HordeEnemy Object Reference"))
  (locals (RandomChoice :type Integer))
  (bind _hordespawns (`self.HordeSpawns`))
  (bind _output_get (set `local.RandomChoice` (`KismetMathLibrary.RandomIntegerInRange` 0 (- (`KismetMathLibrary.Min` (`KismetArrayLibrary.Array_Length` _hordespawns) (+ (/ (`self.MaxAliveEnemies`) 11) 1)) 1))))
  (bind _returnvalue (`self.GetTransform` (`|GetArrayItem` _hordespawns _output_get)))
  (bind _output (`|GetArrayItem` NewParam1 _output_get))
  (bind _returnvalue_2 (`|SpawnActorFromClass` EnemyClass (`KismetMathLibrary.MakeTransform` (`KismetMathLibrary.TransformLocation` _returnvalue (`KismetMathLibrary.MakeVector` (* (/ _output 6) 130.0) (* (mod _output 6) 130.0))) (.rotation _returnvalue)) "Undefined" "OverrideRootScale" null -1 null))
  (`KismetArrayLibrary.Array_Set` NewParam1 _output_get (+ _output 1))
  (return _returnvalue_2))

(fn `SpawnWave`
  (locals (SpawnedPerSpawner :type "Array of Integer") (ChosenWaveVariant :type Integer) (SpawnedPerSpawner :type "Array of Integer"))
  (bind _hordespawns (`self.HordeSpawns`))
  (bind _wave (`self.Wave`))
  (bind _output (`|GetArrayItem` (`self.AIControllers`) (`self.TotalAlive`)))
  (set `self.TotalAlive` 0)
  (bind _asbp_horde_game_state (cast `/Game/Mordhau/Blueprints/GameModes/Horde/BP_HordeGameState` (`GameplayStatics.GetGameState`)))
  (`|ExecutionSequence`
    (:`then_0`
      (set `self.WaveHasSpawned` true)
      (`KismetArrayLibrary.Array_Shuffle` _hordespawns)
      (for _ _hordespawns
        (`KismetArrayLibrary.Array_Add` (`local.SpawnedPerSpawner`))))
    (:`then_1`
      (bind _output_get (set `local.ChosenWaveVariant` (`KismetMathLibrary.RandomInteger` (`KismetArrayLibrary.Array_Length` (`.WaveVariants_12_A13CD2DC46FE272411E9ACAD3C259A2F` (break `/Game/Mordhau/Blueprints/GameModes/Horde/STRUCT_HordeWaveInfo` (`|GetArrayItem` (`self.Waves`) _wave)))))))
      (bind _output_get_2 (set `self.CurrentWaveVariant` (`|GetArrayItem` (`.WaveVariants_12_A13CD2DC46FE272411E9ACAD3C259A2F` (break `/Game/Mordhau/Blueprints/GameModes/Horde/STRUCT_HordeWaveInfo` (`|GetArrayItem` (`self.Waves`) (`self.Wave`)))) _output_get)))
      (set `self.WaveMax` 0)
      (bind _enemies (break `/Game/Mordhau/Blueprints/GameModes/Horde/STRUCT_HordeEnemyArray` _output_get_2))
      (bind _keys (`BlueprintMapLibrary.Map_Keys` _enemies))
      (for _array_element _keys
        (set `self.WaveMax` (+ (`self.WaveMax`) (`BlueprintMapLibrary.Map_Find` _enemies _array_element)))))
    (:`then_2`
      (for _ (range (+ (`KismetMathLibrary.Min` (`self.WaveMax`) (`self.MaxAliveEnemies`)) 1))
        (bind _enemyname (`self.GetEnemyToRespawn`))
        (if (not (== _enemyname "None"))
          (bind (_hordeenemyclsref _equipmentarray _secondaryequipmentarray _botbehaviourclsref _enemyvariantcustomizationactor) (`self.GetCustomizationEnemy` _enemyname))
          (bind _returnvalue (`|GenericCreateObject` _botbehaviourclsref _output))
          (set `MordhauAIController.BehaviorProfile` _returnvalue _output)
          (bind _ascustomization_replication_actor (cast `CustomizationReplicationActor` _enemyvariantcustomizationactor))
          (bind _output_get_3 (set `MordhauAIController.CustomizationReplicationActor` _ascustomization_replication_actor _output))
          (bind _returnvalue_2 (`self.SpawnEnemyActor` _hordeenemyclsref (`local.SpawnedPerSpawner`)))
          (`KismetArrayLibrary.Array_Add` (`self.SpawnedEnemies`) _returnvalue_2)
          (`self.AttachComponentsToEnemy` _output _output_get_3 _equipmentarray _secondaryequipmentarray _returnvalue_2)
          (`/Engine/EditorBlueprintResources/StandardMacros.IncrementInt` (`self.TotalAlive`))))
      (for (_array_element_2 _array_index) (`local.SpawnedPerSpawner`)
        (if (> _array_element_2 0)
          (bind _output_2 (`|GetArrayItem` (`self.HordeSpawns`) _array_index))
          (set `/Game/Mordhau/Blueprints/GameModes/Horde/BP_HordeSpawn.SpawnActivatedCounter` (+ (`/Game/Mordhau/Blueprints/GameModes/Horde/BP_HordeSpawn.SpawnActivatedCounter` _output_2) 1) _output_2))))
    (:`then_3`
      (set `/Game/Mordhau/Blueprints/GameModes/Horde/BP_HordeGameState.ReplicatedHordeMatchInfo` (make `/Game/Mordhau/Blueprints/GameModes/Horde/STRUCT_HordeMatchInfo` (`KismetMathLibrary.Conv_IntToByte` _wave) (`KismetMathLibrary.Conv_IntToByte` (`KismetMathLibrary.Clamp` (`self.WaveMax`) 0 255))) _asbp_horde_game_state))))

(fn `UserConstructionScript`
  (`parent.UserConstructionScript`))
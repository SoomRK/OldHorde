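; Old Horde game state for Mordhau that sets shop and revive prices and shows victory or wave-reached defeat at match end.
; BeginPlay applies class-name default costs, then multicasts server config overrides to purchasables and chests, with OnReps reapplying replicated costs.
; Overrides pair name and cost arrays by index, though AddUnique drops duplicate costs and can misalign them.
; UpdateNextPurchasableVisuals refreshes one purchasable per call, round-robin.
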(event `self.ReceiveBeginPlay`
  (bind _revivepurchase (`self.RevivePurchase`))
  (`|ExecutionSequence`
    (:`then_0`
      (bind _outactors (`GameplayStatics.GetAllActorsOfClass` "/OldHorde/Blueprints/Placeables/BP_RevivePurchase.BP_RevivePurchase_C"))
      (if (> (`KismetArrayLibrary.Array_Length` _outactors) 0)
        (set `self.RevivePurchase` (`|GetArrayItem` _outactors))))
    (:`then_1`
      (`self.GetConfigVar`)
      (`parent.ReceiveBeginPlay`)
      (`KismetSystemLibrary.Delay` 2.0)
      (for _array_element (`self.Purchasables`)
        (bind _asbp_horde_purchasable (cast `/Game/Mordhau/Blueprints/GameModes/Horde/BP_HordePurchasable` _array_element))
        (bind (_value _returnvalue) (`BlueprintMapLibrary.Map_Find` (`self.PurchasableCost`) (`KismetSystemLibrary.GetClassDisplayName` (`GameplayStatics.GetObjectClass` _array_element))))
        (if _returnvalue
          (set `/Game/Mordhau/Blueprints/GameModes/Horde/BP_HordePurchasable.Cost` _value _asbp_horde_purchasable)))
      (`|ExecutionSequence`
        (:`then_0`
          (`/Engine/EditorBlueprintResources/StandardMacros.IsValid` _revivepurchase
            (:`Is Valid`
              (set `/Game/Mordhau/Blueprints/GameModes/Horde/BP_HordePurchasable.Cost` (`self.ReviveCost`) _revivepurchase))))
        (:`then_1`
          (`KismetSystemLibrary.Delay` 0.2)
          (`self.MulticastChangeCosts`))))))

(event `MulticastChangeCosts`
  (if (> (`KismetArrayLibrary.Array_Length` (`self.Overrides`)) 0)
    (for _array_element (`self.Purchasables`)
      (bind _returnvalue (`KismetArrayLibrary.Array_Find` (`self.Overrides`) (`KismetSystemLibrary.GetClassDisplayName` (`GameplayStatics.GetObjectClass` _array_element))))
      (if (not (== _returnvalue -1))
        (bind _asbp_horde_purchasable (cast `/Game/Mordhau/Blueprints/GameModes/Horde/BP_HordePurchasable` _array_element)
          (:`then`
            (bind _output (`|GetArrayItem` (`self.CostArray`) _returnvalue))
            (set `/Game/Mordhau/Blueprints/GameModes/Horde/BP_HordePurchasable.Cost` _output _asbp_horde_purchasable))
          (:`CastFailed`
            (bind _asbp_horde_chest_base (cast `/Game/Mordhau/Blueprints/GameModes/Horde/BP_HordeChestBase` _array_element))
            (set `/Game/Mordhau/Blueprints/GameModes/Horde/BP_HordeChestBase.Cost` _output _asbp_horde_chest_base)))))))

(event `self.HandleMatchEndInfo`
  (`parent.HandleMatchEndInfo`)
  (bind _asbp_mordhau_hud (cast `/Game/Mordhau/Blueprints/BP_MordhauHUD` (`MordhauUtilityLibrary.GetMordhauHUD`)))
  (if (== (`.WinnerTeam_5_6B8C38034236451E9947B38150AA1481` (break `/Game/Mordhau/Blueprints/GameModes/STRUCT_MatchEndInfo` (`self.MatchEndInfo`))) 0)
    (`/Game/Mordhau/Blueprints/BP_MordhauHUD.ShowMatchResult` _asbp_mordhau_hud true "Victory" "")
    (else
      (`/Game/Mordhau/Blueprints/BP_MordhauHUD.ShowMatchResult` _asbp_mordhau_hud false "Defeat" (`|FormatText` "Reached Wave {a}" (+ (`.Wave_8_DA412AC2491458B6B77F2DB0E3CA63A5` (break `/Game/Mordhau/Blueprints/GameModes/Horde/STRUCT_HordeMatchInfo` (`self.ReplicatedHordeMatchInfo`))) 1))))))

(fn `GetConfigVar`
  (bind (_isvalid _returnvalue) (`MordhauUtilityLibrary.GetCustomConfigVar_Int` "OldHorde" "ReviveCost"))
  (bind (_arraysize _returnvalue_2) (`MordhauUtilityLibrary.GetCustomConfigVar_Array` "OldHorde" "ItemCost"))
  (bind (_arraysize_2 _returnvalue_3) (`MordhauUtilityLibrary.GetCustomConfigVar_Array` "OldHorde" "ItemName"))
  (bind _costarray (`self.CostArray`))
  (bind _overrides (`self.Overrides`))
  (`/Engine/EditorBlueprintResources/ActorMacros.Switch Has Authority`
    (:`Authority`
      (`|ExecutionSequence`
        (:`then_0`
          (if (> _arraysize_2 0)
            (if (> _arraysize 0)
              (for _array_element _returnvalue_3
                (`KismetArrayLibrary.Array_AddUnique` _overrides _array_element))
              (for _array_element_2 _returnvalue_2
                (`KismetArrayLibrary.Array_AddUnique` _costarray (`KismetStringLibrary.Conv_StringToInt` _array_element_2)))
              (set `self.Overrides` _overrides)
              (set `self.CostArray` _costarray))))
        (:`then_1`
          (if _isvalid
            (set `self.ReviveCost` _returnvalue)))))))

(fn `OnRep_CostArray`
  (`self.MulticastChangeCosts`))

(fn `OnRep_Overrides`)

(fn `OnRep_ReviveCost`
  (bind _revivepurchase (`self.RevivePurchase`))
  (`/Engine/EditorBlueprintResources/StandardMacros.IsValid` _revivepurchase
    (:`Is Valid`
      (set `/Game/Mordhau/Blueprints/GameModes/Horde/BP_HordePurchasable.Cost` (`self.ReviveCost`) _revivepurchase))))

(fn `OnRep_UseSkillTree`)

(fn `UpdateNextPurchasableVisuals`
  (bind _purchasables (`self.Purchasables`))
  (bind _purchasableindex (`self.PurchasableIndex`))
  (bind _output (`|GetArrayItem` _purchasables _purchasableindex))
  (`|ExecutionSequence`
    (:`then_0`
      (if (not (`KismetArrayLibrary.Array_IsValidIndex` _purchasables _purchasableindex))
        (set `self.PurchasableIndex` 0)))
    (:`then_1`
      (`/Engine/EditorBlueprintResources/StandardMacros.IsValid` _output
        (:`Is Valid`
          (bind _asbp_horde_purchasable (cast `/Game/Mordhau/Blueprints/GameModes/Horde/BP_HordePurchasable` _output)
            (:`then`
              (`/Game/Mordhau/Blueprints/GameModes/Horde/BP_HordePurchasable.UpdateVisuals` _asbp_horde_purchasable))
            (:`CastFailed`
              (bind _asbp_horde_chest_base (cast `/Game/Mordhau/Blueprints/GameModes/Horde/BP_HordeChestBase` _output))
              (`/Game/Mordhau/Blueprints/GameModes/Horde/BP_HordeChestBase.UpdateVisuals` _asbp_horde_chest_base))))))
    (:`then_2`
      (set `self.PurchasableIndex` (+ (`self.PurchasableIndex`) 1)))))

(fn `UserConstructionScript`
  (`parent.UserConstructionScript`))
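; Horde mode player controller that lets players gift gold to each other, with empty AFK-kick overrides.
; It registers an F5 "Gift" binding at runtime, which gathers player names and opens the HUD gift widget, whose options refresh through an OnRep.
; GiftGold deducts coins, credits the first name or substring match, and reports in chat.
; Other OnReps play bonus and revive sounds; an uncalled helper dumps chest item lists to files.
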(event `self.ReceiveBeginPlay`
  (`parent.ReceiveBeginPlay`)
  (`/Engine/EditorBlueprintResources/StandardMacros.IsValid` (`MordhauUtilityLibrary.GetMordhauInput`) :!label _label
    (:`Is Valid`
      (`self.AddMordhauInput` (make `InputActionKeyMapping` "Gift" false false false false "F5")))
    (:`Is Not Valid`
      (`KismetSystemLibrary.Delay` 2.0)
      (goto _label))))

(event `GiftGold`
  (params (`Player Name` :type Text) (GoldToGive :type Integer))
  (bind _success (`self.SpendCoins` GoldToGive))
  (if _success
    (bind (_player_state _found) (`self.FindPlayer` `Player Name`))
    (if _found
      (bind _asbp_horde_player_state (cast `/Game/Mordhau/Blueprints/GameModes/Horde/BP_HordePlayerState` _player_state))
      (set `/Game/Mordhau/Blueprints/GameModes/Horde/BP_HordePlayerState.Coins` (+ (`/Game/Mordhau/Blueprints/GameModes/Horde/BP_HordePlayerState.Coins` _asbp_horde_player_state) GoldToGive) _asbp_horde_player_state)
      (`self.RequestChatMessage` (`KismetStringLibrary.Concat_StrStr` "Has Given " (`KismetStringLibrary.Conv_IntToString` GoldToGive) " Gold to " (`KismetTextLibrary.Conv_TextToString` `Player Name`)))
      (else
        (`self.RequestChatMessage` "This player does not exist")))
    (else
      (`self.RequestChatMessage` "I do not have enough Gold to Give"))))

(event `self.OnAFKTimeExceededMaximum`)

(event `self.PerformAFKKick`)

(event `InputAction|Gift`
  (params (Key :type "Key Structure"))
  (:`Pressed`
    (`self.GetPlayers`)
    (bind _asbp_old_horde_hud (cast `/OldHorde/Blueprints/BP_OldHordeHUD` (`self.GetHUD`)))
    (`/OldHorde/Blueprints/BP_OldHordeHUD.ShowGoldGifts` _asbp_old_horde_hud)))

(fn `AddMordhauInput`
  (params (`Input Action` :type "InputActionKeyMapping Structure"))
  (returns (Success :type Boolean))
  (locals (AlreadyExists :type Boolean))
  (bind _returnvalue (`MordhauUtilityLibrary.GetMordhauInput`))
  (bind _actionmappings (`MordhauInput.ActionMappings` _returnvalue))
  ;[1 1 1] NOTE: You need to make Input action inside Unreal Project settings to be able to get the event for this input action
  (for _array_element _actionmappings
    (if (== (`.ActionName` (break `InputActionKeyMapping` _array_element)) (`.ActionName` (break `InputActionKeyMapping` `Input Action`)))
      (set `local.AlreadyExists` true)
      (break)))
  (if (`local.AlreadyExists`)
    (return false)
    (else
      (`KismetArrayLibrary.Array_Add` _actionmappings `Input Action`)
      (`MordhauInput.SaveSettings` _returnvalue)
      (`MordhauInput.ApplySettings` _returnvalue)
      (return true))))

(fn `FindPlayer`
  (params (`Player Name` :type Text))
  (returns (`Player State` :type "PlayerState Object Reference") (Found :type Boolean))
  (locals (NewLocalVar_0 :type "/Game/Mordhau/Blueprints/GameModes/Horde/BP_HordePlayerState Object Reference"))
  (bind _returnvalue (`KismetTextLibrary.Conv_TextToString` `Player Name`))
  (bind _giftplayerstate (`self.GiftPlayerState`))
  (set `self.GiftPlayerState` null)
  (bind _asbp_horde_game_state (cast `/Game/Mordhau/Blueprints/GameModes/Horde/BP_HordeGameState` (`GameplayStatics.GetGameState`)))
  (for _array_element (`GameStateBase.PlayerArray` _asbp_horde_game_state)
    (bind _asbp_horde_player_state (cast `/Game/Mordhau/Blueprints/GameModes/Horde/BP_HordePlayerState` _array_element))
    (bind _returnvalue_2 (`PlayerState.GetPlayerName` _asbp_horde_player_state))
    (if (or (`KismetStringLibrary.Contains` _returnvalue_2 _returnvalue) (`KismetStringLibrary.EqualEqual_StrStr` _returnvalue_2 _returnvalue))
      (set `self.GiftPlayerState` _asbp_horde_player_state)
      (break)))
  (return _giftplayerstate (not (== _giftplayerstate null))))

(fn `GetPlayers`
  (bind _target_array (`self.Target Array`))
  (bind _asbp_horde_game_state (cast `/Game/Mordhau/Blueprints/GameModes/Horde/BP_HordeGameState` (`GameplayStatics.GetGameState`)))
  (for (_array_element _array_index) (`GameStateBase.PlayerArray` _asbp_horde_game_state)
    (`/Engine/EditorBlueprintResources/StandardMacros.IsValid` _array_element
      (:`Is Valid`
        (bind _asbp_horde_player_state (cast `/Game/Mordhau/Blueprints/GameModes/Horde/BP_HordePlayerState` _array_element))
        (`KismetArrayLibrary.Array_Set` _target_array _array_index (`PlayerState.GetPlayerName` _asbp_horde_player_state) true))))
  (set `self.Target Array` _target_array))

(fn `NewFunction_1`
  (locals (NewLocalVar_1 :type String) (NewLocalVar_2 :type "Array of Float (double-precision)") (NewLocalVar_0 :type String))
  (bind _asbp_horde_game_state (cast `/Game/Mordhau/Blueprints/GameModes/Horde/BP_HordeGameState` (`GameplayStatics.GetGameState`)))
  (for _array_element (`/Game/Mordhau/Blueprints/GameModes/Horde/BP_HordeGameState.Purchasables` _asbp_horde_game_state)
    (bind _asbp_horde_chest_base (cast `/Game/Mordhau/Blueprints/GameModes/Horde/BP_HordeChestBase` _array_element))
    (set `local.NewLocalVar_1` (`KismetSystemLibrary.GetDisplayName` _asbp_horde_chest_base))
    (bind _itemlist (`/Game/Mordhau/Blueprints/GameModes/BattleRoyale/BP_BattleRoyaleBaseItemSpawn.ItemList` _asbp_horde_chest_base))
    (bind _keys (`BlueprintMapLibrary.Map_Keys` _itemlist))
    (bind _values (`BlueprintMapLibrary.Map_Values` _itemlist))
    (set `local.NewLocalVar_2` _values)
    (for (_array_element_2 _array_index) _keys
      (bind _asmordhau_equipment (castclass `MordhauEquipment` _array_element_2))
      (set `local.NewLocalVar_0` (`KismetStringLibrary.Concat_StrStr` (`local.NewLocalVar_0`) " \n" (`KismetStringLibrary.Concat_StrStr` (`KismetTextLibrary.Conv_TextToString` (`.EquipmentName` (defaults `Object` _asmordhau_equipment))) " == " (`KismetStringLibrary.Conv_DoubleToString` (`|GetArrayItem` _values _array_index))))))
    (`MordhauUtilityLibrary.SaveStringToFile` (`local.NewLocalVar_1`) (`local.NewLocalVar_0`))))

(fn `OnRep_GoldBonus`
  (`/Engine/EditorBlueprintResources/StandardMacros.Can Execute Cosmetic Events`
    (:`True`
      (`GameplayStatics.PlaySound2D` "/Game/Mordhau/Audio/Cues/Misc/SC_CoinObjective.SC_CoinObjective" 1.0 1.0 0.0 null null))))

(fn `OnRep_ReviveCounter`
  (`/Engine/EditorBlueprintResources/StandardMacros.Can Execute Cosmetic Events`
    (:`True`
      (`GameplayStatics.PlaySound2D` "/Game/Mordhau/Audio/Cues/Horde/Abilities/Soundcues/SC_ABL_DivineFavor.SC_ABL_DivineFavor" 0.8 1.0 0.0 null null))))

(fn `OnRep_Target Array`
  (bind _asbp_old_horde_hud (cast `/OldHorde/Blueprints/BP_OldHordeHUD` (`self.GetHUD`)))
  (bind _options (`/OldHorde/Blueprints/BP_GoldGiftWidget.Options` (`/OldHorde/Blueprints/BP_OldHordeHUD.GoldWidget` _asbp_old_horde_hud)))
  (`KismetArrayLibrary.Array_Clear` _options)
  (for _array_element (`self.Target Array`)
    (`KismetArrayLibrary.Array_AddUnique` _options (`KismetTextLibrary.Conv_StringToText` _array_element))))

(fn `SpendCoins`
  (params (Amount :type Integer))
  (returns (Success :type Boolean))
  (`|ExecutionSequence`
    (:`then_0`
      (bind _asbp_horde_player_state (cast `/Game/Mordhau/Blueprints/GameModes/Horde/BP_HordePlayerState` (`self.PlayerState`)))
      (bind _coins (`/Game/Mordhau/Blueprints/GameModes/Horde/BP_HordePlayerState.Coins` _asbp_horde_player_state))
      (if (>= _coins Amount)
        (set `/Game/Mordhau/Blueprints/GameModes/Horde/BP_HordePlayerState.Coins` (- _coins Amount) _asbp_horde_player_state)
        (set `self.PurchaseTrigger` (+ (`self.PurchaseTrigger`) 1))
        (return true)))
    (:`then_1`
      (return false))))

(fn `UserConstructionScript`
  (`parent.UserConstructionScript`))
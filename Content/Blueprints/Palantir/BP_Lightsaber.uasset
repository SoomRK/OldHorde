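; BP_Lightsaber is a lightsaber weapon Blueprint that extends a parent weapon's equip, holster and fire events.
; Equipping activates and plays a looping Jedi saber audio cue, and holstering stops and deactivates it.
; After each parent FireProjectile call, it waits briefly and resets ammo to one if it differs, so the weapon never runs dry.
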(event `self.OnEquipped`
  (params (Character :type "MordhauCharacter Object Reference"))
  (bind _ls_jedi_active_loop_cue (`self.ls_jedi_active_loop_Cue`))
  (`parent.OnEquipped` Character)
  (`ActorComponent.Activate` _ls_jedi_active_loop_cue true)
  (`AudioComponent.Play` _ls_jedi_active_loop_cue 0.0))

(event `self.OnHolstered`
  (params (Character :type "MordhauCharacter Object Reference"))
  (bind _ls_jedi_active_loop_cue (`self.ls_jedi_active_loop_Cue`))
  (`parent.OnHolstered` Character)
  (`AudioComponent.Stop` _ls_jedi_active_loop_cue)
  (`ActorComponent.Deactivate` _ls_jedi_active_loop_cue))

(event `self.FireProjectile`
  (params (Origin :type "Vector Structure (by ref)") (Orientation :type "Rotator Structure (by ref)") (OwningController :type "Controller Object Reference") (ExpectedDelay :type "Float (single-precision)"))
  (`parent.FireProjectile` Origin Orientation OwningController ExpectedDelay)
  (`KismetSystemLibrary.Delay` 1.0)
  (if (not (== (`self.GetAmmo`) 1))
    (`self.SetAmmo` 1)))

(fn `UserConstructionScript`
  (`parent.UserConstructionScript`))
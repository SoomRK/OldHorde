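; Horde-mode player controller for the Seymour Palantir map that swaps streamed map instances (Taiga, Cortile, Mountain) by wave band.
; BeginPlay loads the local player's map for the current wave, and RoundEnded triggers switches at waves 5 and 10.
; Each switch fades the camera, clears the current level and retries failed loads.
; Looping timers keep requesting unload of the previous map until it is gone.
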(event `self.ReceiveBeginPlay`
  (`parent.ReceiveBeginPlay`)
  (`KismetSystemLibrary.Delay` 2.0)
  (bind _asbp_old_horde_game_state_seymour (cast `/OldHorde/Blueprints/Palantir/BP_OldHordeGameState_Seymour` (`GameplayStatics.GetGameState`)))
  (if (`self.IsLocalPlayerController`)
    (bind _returnvalue (+ (`/OldHorde/Blueprints/Palantir/BP_OldHordeGameState_Seymour.CurrentWave` _asbp_old_horde_game_state_seymour) 1))
    (`KismetSystemLibrary.PrintString` (`KismetStringLibrary.Conv_IntToString` _returnvalue))
    (switch `int` _returnvalue
      (:`0`
        (`self.FadeCamera` :!label _label)
        (`KismetSystemLibrary.Delay` 1.0)
        (bind (_boutsuccess _returnvalue_2) (`LevelStreamingDynamic.LoadLevelInstanceBySoftObjectPtr` "/PalantirOfSeymour/PalantirOfSeymour_Taiga.PalantirOfSeymour_Taiga" :!label _label_2))
        (if _boutsuccess
          (bind _output_get (set `self.Taiga` _returnvalue_2))
          (set `LevelStreaming.bShouldBlockOnLoad` false _output_get)
          (set `LevelStreaming.bShouldBeVisible` true _output_get)
          (else
            (`KismetSystemLibrary.Delay` 1.0)
            (goto _label_2))))
      (:`1`
        (goto _label))
      (:`2`
        (goto _label))
      (:`3`
        (goto _label))
      (:`4`
        (goto _label))
      (:`5`
        (`self.FadeCamera` :!label _label_3)
        (`KismetSystemLibrary.Delay` 1.0)
        (`self.ClearLevel` :!label _label_4)
        (`KismetSystemLibrary.Delay` 0.2)
        (bind (_boutsuccess_2 _returnvalue_3) (`LevelStreamingDynamic.LoadLevelInstanceBySoftObjectPtr` "/PalantirOfSeymour/PalantirOfSeymour_Cortile.PalantirOfSeymour_Cortile"))
        (if _boutsuccess_2
          (bind _output_get_2 (set `self.Cortile` _returnvalue_3))
          (set `LevelStreaming.bShouldBeVisible` true _output_get_2)
          (set `LevelStreaming.bShouldBlockOnLoad` false _output_get_2)
          (`KismetSystemLibrary.Delay` 1.0 :!label _label_5)
          (bind _returnvalue_4 (`KismetSystemLibrary.K2_SetTimerDelegate` (delegate `Unload1stMap_Timer`) 2.0 true))
          (set `self.NewVar_2` _returnvalue_4)
          (else
            (`KismetSystemLibrary.Delay` 1.0)
            (goto _label_4))))
      (:`6`
        (goto _label_3))
      (:`7`
        (goto _label_3))
      (:`8`
        (goto _label_3))
      (:`9`
        (goto _label_3))
      (:`10`
        (`self.FadeCamera` :!label _label_6)
        (`KismetSystemLibrary.Delay` 1.0)
        (`self.ClearLevel` :!label _label_7)
        (`KismetSystemLibrary.Delay` 0.2)
        (bind (_boutsuccess_3 _returnvalue_5) (`LevelStreamingDynamic.LoadLevelInstanceBySoftObjectPtr` "/PalantirOfSeymour/PalantirOfSeymour_Mountain.PalantirOfSeymour_Mountain"))
        (if _boutsuccess_3
          (bind _output_get_3 (set `self.Mountain` _returnvalue_5))
          (set `LevelStreaming.bShouldBeVisible` true _output_get_3)
          (set `LevelStreaming.bShouldBlockOnLoad` false _output_get_3)
          (`KismetSystemLibrary.Delay` 1.0 :!label _label_8)
          (bind _returnvalue_6 (`KismetSystemLibrary.K2_SetTimerDelegate` (delegate `Unload2ndMap_Timer`) 2.0 true))
          (set `self.NewVar_1` _returnvalue_6)
          (else
            (`KismetSystemLibrary.Delay` 1.0)
            (goto _label_7))))
      (:`11`
        (goto _label_6))
      (:`12`
        (goto _label_6))
      (:`13`
        (goto _label_6))
      (:`14`
        (goto _label_6))
      (:`15`
        (goto _label_6)))))

(event `Unload1stMap_Timer`
  (bind _taiga (`self.Taiga`))
  (`/Engine/EditorBlueprintResources/StandardMacros.IsValid` _taiga
    (:`Is Valid`
      (`LevelStreaming.SetIsRequestingUnloadAndRemoval` _taiga true)
      (`GameplayStatics.UnloadStreamLevelBySoftObjectPtr` (`LevelStreaming.WorldAsset` _taiga)))
    (:`Is Not Valid`
      (`KismetSystemLibrary.K2_ClearAndInvalidateTimerHandle` (`self.NewVar_2`))
      (`GameplayStatics.UnloadStreamLevelBySoftObjectPtr` "/PalantirOfSeymour/PalantirOfSeymour_Taiga.PalantirOfSeymour_Taiga"))))

(event `Unload2ndMap_Timer`
  (bind _cortile (`self.Cortile`))
  (`/Engine/EditorBlueprintResources/StandardMacros.IsValid` _cortile
    (:`Is Valid`
      (`LevelStreaming.SetIsRequestingUnloadAndRemoval` _cortile true)
      (`GameplayStatics.UnloadStreamLevelBySoftObjectPtr` (`LevelStreaming.WorldAsset` _cortile)))
    (:`Is Not Valid`
      (`KismetSystemLibrary.K2_ClearAndInvalidateTimerHandle` (`self.NewVar_1`))
      (`GameplayStatics.UnloadStreamLevelBySoftObjectPtr` "/PalantirOfSeymour/PalantirOfSeymour_Cortile.PalantirOfSeymour_Cortile"))))

(event `TriggerLevelChange`
  (bind _asbp_old_horde_game_state_seymour (cast `/OldHorde/Blueprints/Palantir/BP_OldHordeGameState_Seymour` (`GameplayStatics.GetGameState`)))
  (bind _returnvalue (+ (`/OldHorde/Blueprints/Palantir/BP_OldHordeGameState_Seymour.CurrentWave` _asbp_old_horde_game_state_seymour) 1))
  (`KismetSystemLibrary.PrintString` (`KismetStringLibrary.Conv_IntToString` _returnvalue))
  (switch `int` _returnvalue
    (:`5`
      (`self.FadeCamera`)
      (`KismetSystemLibrary.Delay` 1.0)
      (`self.ClearLevel` :!label _label_9)
      (`KismetSystemLibrary.Delay` 0.2)
      (bind (_boutsuccess _returnvalue_2) (`LevelStreamingDynamic.LoadLevelInstanceBySoftObjectPtr` "/PalantirOfSeymour/PalantirOfSeymour_Cortile.PalantirOfSeymour_Cortile"))
      (if _boutsuccess
        (bind _output_get (set `self.Cortile` _returnvalue_2))
        (set `LevelStreaming.bShouldBlockOnLoad` false _output_get)
        (set `LevelStreaming.bShouldBeVisible` true _output_get)
        (goto _label_5)
        (else
          (`KismetSystemLibrary.Delay` 1.0)
          (goto _label_9))))
    (:`10`
      (`self.FadeCamera`)
      (`KismetSystemLibrary.Delay` 1.0)
      (`self.ClearLevel` :!label _label_10)
      (`KismetSystemLibrary.Delay` 0.2)
      (bind (_boutsuccess_2 _returnvalue_3) (`LevelStreamingDynamic.LoadLevelInstanceBySoftObjectPtr` "/PalantirOfSeymour/PalantirOfSeymour_Mountain.PalantirOfSeymour_Mountain"))
      (if _boutsuccess_2
        (bind _output_get_2 (set `self.Mountain` _returnvalue_3))
        (set `LevelStreaming.bShouldBlockOnLoad` false _output_get_2)
        (set `LevelStreaming.bShouldBeVisible` true _output_get_2)
        (goto _label_8)
        (else
          (`KismetSystemLibrary.Delay` 1.0)
          (goto _label_10))))))

(event `FadeCamera`
  (`PlayerCameraManager.StartCameraFade` :`self` (`self.PlayerCameraManager`) :`ToAlpha` 2.0 :`Duration` 2.0 :`bHoldWhenFinished` true)
  (`KismetSystemLibrary.Delay` 2.0)
  (`PlayerCameraManager.StartCameraFade` :`self` (`self.PlayerCameraManager`) :`FromAlpha` 2.0 :`Duration` 2.0 :`bHoldWhenFinished` true))

(event `self.ReceiveEndPlay`
  (params (EndPlayReason :type "EEndPlayReason Enum" :default "Destroyed"))
  (`self.ClearLevel`)
  (`parent.ReceiveEndPlay` EndPlayReason))

(event `ClearLevel`
  (bind _mountain (`self.Mountain`))
  (bind _cortile (`self.Cortile`))
  (bind _taiga (`self.Taiga`))
  (`/Engine/EditorBlueprintResources/StandardMacros.IsValid` _taiga
    (:`Is Valid`
      (`LevelStreaming.SetIsRequestingUnloadAndRemoval` _taiga true)
      (`GameplayStatics.UnloadStreamLevelBySoftObjectPtr` (`LevelStreaming.WorldAsset` _taiga)))
    (:`Is Not Valid`
      (`/Engine/EditorBlueprintResources/StandardMacros.IsValid` _cortile
        (:`Is Valid`
          (`LevelStreaming.SetIsRequestingUnloadAndRemoval` _cortile true)
          (`GameplayStatics.UnloadStreamLevelBySoftObjectPtr` (`LevelStreaming.WorldAsset` _cortile)))
        (:`Is Not Valid`
          (`/Engine/EditorBlueprintResources/StandardMacros.IsValid` _mountain
            (:`Is Valid`
              (`LevelStreaming.SetIsRequestingUnloadAndRemoval` _mountain true)
              (`GameplayStatics.UnloadStreamLevelBySoftObjectPtr` (`LevelStreaming.WorldAsset` _mountain)))))))))

(fn `OnRep_EyeBlink`)

(fn `RoundEnded`
  (`self.TriggerLevelChange`))

(fn `UserConstructionScript`
  (`parent.UserConstructionScript`))
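; BP_OldHordeHUD_Seymour is a horde mode HUD variant that installs the Seymour old-style horde HUD widget.
; When the game state replicates, it runs the parent logic, then removes the existing horde widget and creates BP_OldHordeHUDWidget_Seymour with the skill tree enabled.
; The new widget is added to the viewport behind default layers and collapsed if the HUD is in minimal mode.
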(event `self.OnGameStateReplicated`
  (`parent.OnGameStateReplicated`)
  (`Widget.RemoveFromParent` (`self.HordeHUDWidget`))
  (set `self.HordeHUDWidget` null)
  (bind _returnvalue (`|CreateWidget` "/OldHorde/Blueprints/BP_OldHordeHUDWidget_Seymour.BP_OldHordeHUDWidget_Seymour_C" (`GameplayStatics.GetPlayerController` 0) true))
  (bind _output_get (set `self.HordeHUDWidget` _returnvalue))
  (`UserWidget.AddToViewport` _output_get -5)
  (if (`self.IsHUDMinimal`)
    (`Widget.SetVisibility` _output_get "Collapsed")))

(fn `UserConstructionScript`
  (`parent.UserConstructionScript`))
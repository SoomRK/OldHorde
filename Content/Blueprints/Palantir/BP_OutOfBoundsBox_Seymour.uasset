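; Out-of-bounds volume for Horde mode that notifies horde characters when they enter or leave it and periodically damages idle horde enemies inside.
; A looping 22-second timer deals generic damage to overlapping BP_HordeEnemy actors whose current motion is IdleMotion.
; A second looping timer polls the Disabled flag every few seconds to pause or resume the damage timer, which is cleared on EndPlay.
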(event `self.ReceiveEndPlay`
  (params (EndPlayReason :type "EEndPlayReason Enum" :default "Destroyed"))
  (`parent.ReceiveEndPlay` EndPlayReason)
  (`KismetSystemLibrary.K2_ClearAndInvalidateTimerHandle` (`self.Timer`)))

(event `self.ReceiveBeginPlay`
  (bind _returnvalue (`KismetSystemLibrary.K2_SetTimerDelegate` (delegate `CustomEvent_0`) 22.0 true))
  (set `self.Timer` _returnvalue)
  (`KismetSystemLibrary.K2_SetTimerDelegate` (delegate `CustomEvent_2`) 5.0 true))

(event `CustomEvent_3`
  (bind _timer (`self.Timer`))
  (if (`self.Disabled`)
    (`KismetSystemLibrary.K2_PauseTimerHandle` _timer)
    (else
      (`KismetSystemLibrary.K2_UnPauseTimerHandle` _timer))))

(event `CustomEvent_0`
  (`self.CustomEvent_1`))

(event `CustomEvent_2`
  (`self.CustomEvent_3`))

(event `CustomEvent_1`
  (if (not (`self.Disabled`))
    (for _array_element (`PrimitiveComponent.GetOverlappingActors` (`self.Box`) "/Game/Mordhau/Blueprints/GameModes/Horde/BP_HordeEnemy.BP_HordeEnemy_C")
      (bind _asbp_horde_enemy (cast `/Game/Mordhau/Blueprints/GameModes/Horde/BP_HordeEnemy` _array_element))
      (cast `IdleMotion` (`AdvancedCharacter.GetMotion` _asbp_horde_enemy))
      (`AdvancedCharacter.MordhauTakeDamage` _asbp_horde_enemy 69.0 (`GameplayStatics.MakeHitResult` false) "Generic" 0 self null null))))

(event `self.ReceiveActorEndOverlap`
  (params (OtherActor :type "Actor Object Reference"))
  (bind _asbp_horde_character (cast `/Game/Mordhau/Blueprints/Characters/BP_HordeCharacter` OtherActor))
  (message `Bounds.LeftOutOfBoundsArea` _asbp_horde_character))

(event `self.ReceiveActorBeginOverlap`
  (params (OtherActor :type "Actor Object Reference"))
  (bind _asbp_horde_character (cast `/Game/Mordhau/Blueprints/Characters/BP_HordeCharacter` OtherActor))
  (message `Bounds.EnteredOutOfBoundsArea` _asbp_horde_character self))

(fn `UserConstructionScript`)
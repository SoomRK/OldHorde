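; Horde game state for the Palantir of Seymour that streams Taiga, Cortile and Mountain level instances as waves progress.
; BeginPlay loads the stage matching CurrentWave; a wave-progress multicast, gated on the match being in progress, swaps stages at thresholds after a local camera fade.
; The multicast also destroys MasterField actors in late waves, and EndPlay unloads all stages.
; Out-of-bounds toggling, spawn gathering and CurrentWave assignment are left unwired.
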(event `self.ReceiveBeginPlay`
  (`parent.ReceiveBeginPlay`)
  (add `self.ProgressWave` (delegate `ProgressWave_Event`))
  (switch `int` (`self.CurrentWave`)
    (:`0`
      (`self.NewFunction_0` 0 :!label _label)
      (`KismetSystemLibrary.Delay` 1.5)
      (bind (_boutsuccess _returnvalue) (`LevelStreamingDynamic.LoadLevelInstanceBySoftObjectPtr` "/PalantirOfSeymour/PalantirOfSeymour_Taiga.PalantirOfSeymour_Taiga"))
      (set `self.Taiga` _returnvalue))
    (:`1`
      (goto _label))
    (:`2`
      (goto _label))
    (:`3`
      (goto _label))
    (:`4`
      (goto _label))
    (:`5`
      (`self.NewFunction_0` 5 :!label _label_2)
      (`KismetSystemLibrary.Delay` 1.5)
      (`LevelStreaming.SetIsRequestingUnloadAndRemoval` (`self.Taiga`) true)
      (bind (_boutsuccess_2 _returnvalue_2) (`LevelStreamingDynamic.LoadLevelInstanceBySoftObjectPtr` "/PalantirOfSeymour/PalantirOfSeymour_Cortile.PalantirOfSeymour_Cortile"))
      (set `self.Cortile` _returnvalue_2))
    (:`6`
      (goto _label_2))
    (:`7`
      (goto _label_2))
    (:`8`
      (goto _label_2))
    (:`9`
      (goto _label_2))
    (:`10`
      (`self.NewFunction_0` 10 :!label _label_3)
      (`KismetSystemLibrary.Delay` 1.5)
      (`LevelStreaming.SetIsRequestingUnloadAndRemoval` (`self.Cortile`) true)
      (bind (_boutsuccess_3 _returnvalue_3) (`LevelStreamingDynamic.LoadLevelInstanceBySoftObjectPtr` "/PalantirOfSeymour/PalantirOfSeymour_Mountain.PalantirOfSeymour_Mountain"))
      (set `self.Mountain` _returnvalue_3))
    (:`11`
      (goto _label_3))
    (:`12`
      (goto _label_3))
    (:`13`
      (goto _label_3))
    (:`14`
      (goto _label_3))
    (:`15`
      (goto _label_3))))

(event `ProgressWave_Event` :!signature `self.ProgressWave`
  (params (Wave :type Integer))
  (`self.Mutlicast_ProgressWave` Wave))

(event `self.ReceiveTick`
  (params (DeltaSeconds :type "Float (single-precision)"))
  (`parent.ReceiveTick` DeltaSeconds)
  (if (== (`self.MatchState`) "InProgress")
    (`/Engine/EditorBlueprintResources/StandardMacros.DoOnce` false
      (:`Completed`
        (set `self.Condition` true)))
    (else
      (set `self.Condition` false))))

(event `Mutlicast_ProgressWave`
  (params (Wave :type Integer))
  (if (`self.Condition`)
    (`|ExecutionSequence`
      (:`then_0`
        (switch `int` Wave
          (:`0`
            (`self.NewFunction_0` 0)
            (`KismetSystemLibrary.Delay` 1.5)
            (bind (_boutsuccess _returnvalue) (`LevelStreamingDynamic.LoadLevelInstanceBySoftObjectPtr` "/PalantirOfSeymour/PalantirOfSeymour_Taiga.PalantirOfSeymour_Taiga"))
            (bind _output_get (set `self.Taiga` _returnvalue))
            (set `LevelStreaming.bShouldBlockOnLoad` true _output_get))
          (:`5`
            (`self.NewFunction_0` 5)
            (`KismetSystemLibrary.Delay` 1.5)
            (`LevelStreaming.SetIsRequestingUnloadAndRemoval` (`self.Taiga`) true)
            (bind (_boutsuccess_2 _returnvalue_2) (`LevelStreamingDynamic.LoadLevelInstanceBySoftObjectPtr` "/PalantirOfSeymour/PalantirOfSeymour_Cortile.PalantirOfSeymour_Cortile"))
            (bind _output_get_2 (set `self.Cortile` _returnvalue_2))
            (set `LevelStreaming.bShouldBlockOnLoad` true _output_get_2))
          (:`10`
            (`self.NewFunction_0` 10)
            (`KismetSystemLibrary.Delay` 1.5)
            (`LevelStreaming.SetIsRequestingUnloadAndRemoval` (`self.Cortile`) true)
            (bind (_boutsuccess_3 _returnvalue_3) (`LevelStreamingDynamic.LoadLevelInstanceBySoftObjectPtr` "/PalantirOfSeymour/PalantirOfSeymour_Mountain.PalantirOfSeymour_Mountain"))
            (bind _output_get_3 (set `self.Mountain` _returnvalue_3))
            (set `LevelStreaming.bShouldBlockOnLoad` true _output_get_3))))
      (:`then_1`
        (if (>= (`self.CurrentWave`) 13)
          (bind _outactors (`GameplayStatics.GetAllActorsOfClass` "/Game/Mordhau/Blueprints/Fields/BP_MasterField.BP_MasterField_C"))
          (if (> (`KismetArrayLibrary.Array_Length` _outactors) 0)
            (for _array_element _outactors
              (`self.SetReplicates` _array_element true)
              (`self.K2_DestroyActor` _array_element))))))))

(event `self.ReceiveEndPlay`
  (params (EndPlayReason :type "EEndPlayReason Enum" :default "Destroyed"))
  (bind _mountain (`self.Mountain`))
  (bind _taiga (`self.Taiga`))
  (bind _cortile (`self.Cortile`))
  (`|ExecutionSequence`
    (:`then_0`
      (`|ExecutionSequence`
        (:`then_0`
          (`/Engine/EditorBlueprintResources/StandardMacros.IsValid` _taiga
            (:`Is Valid`
              (`LevelStreaming.SetIsRequestingUnloadAndRemoval` _taiga true))))
        (:`then_1`
          (`/Engine/EditorBlueprintResources/StandardMacros.IsValid` _cortile
            (:`Is Valid`
              (`LevelStreaming.SetIsRequestingUnloadAndRemoval` _cortile true))))
        (:`then_2`
          (`/Engine/EditorBlueprintResources/StandardMacros.IsValid` _mountain
            (:`Is Valid`
              (`LevelStreaming.SetIsRequestingUnloadAndRemoval` _mountain true))))))
    (:`then_1`
      (`parent.ReceiveEndPlay` EndPlayReason))))

(fn `NewFunction_0`
  (params (NewParam :type Integer))
  (bind _returnvalue (`GameplayStatics.GetPlayerController` 0))
  (`/Engine/EditorBlueprintResources/StandardMacros.IsValid` _returnvalue
    (:`Is Valid`
      (if (`Controller.IsLocalPlayerController` _returnvalue)
        (bind _asbp_old_horde_player_controller_seymour (cast `/OldHorde/Blueprints/Palantir/BP_OldHordePlayerController_Seymour` _returnvalue))
        (`/OldHorde/Blueprints/Palantir/BP_OldHordePlayerController_Seymour.FadeCamera` _asbp_old_horde_player_controller_seymour)))))

(fn `OnRep_CurrentWave`)

(fn `ToggleOOB`
  (params (Disabled :type Boolean))
  (locals (Temp :type Boolean))
  (set `local.Temp` Disabled)
  (bind _outactors (`GameplayStatics.GetAllActorsOfClass` "/OldHorde/Blueprints/Palantir/BP_OutOfBoundsBox_Seymour.BP_OutOfBoundsBox_Seymour_C"))
  (for _array_element _outactors
    (set `/OldHorde/Blueprints/Palantir/BP_OutOfBoundsBox_Seymour.Disabled` (`local.Temp`) _array_element)))

(fn `UserConstructionScript`
  (`parent.UserConstructionScript`))
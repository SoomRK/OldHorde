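; Game mode for the Seymour variant of Old Horde, a wave-based mode built on a parent horde game mode.
; On each wave change it calls RoundEnded on its player controllers and passes the wave number to the game state.
; It pre-spawns a pool of AI controllers sized to the alive-enemy cap.
; GetConfig reads OldHorde custom config for team damage, wave timing, selling, explosives and player scaling, writing back only a missing team-damage default.
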(event `self.ReceiveBeginPlay`
  (`parent.ReceiveBeginPlay`))

(event `self.OnKilled`
  (params (Killer :type "Controller Object Reference") (KilledPlayer :type "Controller Object Reference") (KilledPawn :type "Pawn Object Reference") (Type :type "EMordhauDamageType Enum" :default "Generic") (SubType :type Byte) (DamageSource :type "Actor Object Reference") (DamageAgent :type "Actor Object Reference"))
  (`parent.OnKilled` Killer KilledPlayer KilledPawn Type SubType DamageSource DamageAgent))

(event `self.ProgressWave`
  (bind _wave (`self.Wave`))
  (`parent.ProgressWave`)
  (bind _outactors (`GameplayStatics.GetAllActorsOfClass` "/OldHorde/Blueprints/Palantir/BP_OldHordePlayerController_Seymour.BP_OldHordePlayerController_Seymour_C"))
  (for _array_element _outactors
    (`/OldHorde/Blueprints/Palantir/BP_OldHordePlayerController_Seymour.RoundEnded` _array_element))
  (bind _asbp_old_horde_game_state_seymour (cast `/OldHorde/Blueprints/Palantir/BP_OldHordeGameState_Seymour` (`GameplayStatics.GetGameState`)))
  (set `/OldHorde/Blueprints/Palantir/BP_OldHordeGameState_Seymour.CurrentWave` _wave _asbp_old_horde_game_state_seymour)
  (`/OldHorde/Blueprints/Palantir/BP_OldHordeGameState_Seymour.ProgressWave` _asbp_old_horde_game_state_seymour _wave))

(event `self.HealTeamOnServer`
  (`parent.HealTeamOnServer`))

(event `self.HealTeam`
  (params (Character :type "/Game/Mordhau/Blueprints/Characters/BP_HordeCharacter Object Reference"))
  (`parent.HealTeam` Character))

(event `self.K2_PostLogin`
  (params (NewPlayer :type "PlayerController Object Reference"))
  (`parent.K2_PostLogin` NewPlayer))

(fn `GetConfig`
  (returns (IsValid :type Boolean))
  (bind (_isvalid _returnvalue) (`MordhauUtilityLibrary.GetCustomConfigVar_Float` "OldHorde" "TimeBetweenWaves"))
  (bind (_isvalid_2 _returnvalue_2) (`MordhauUtilityLibrary.GetCustomConfigVar_Bool` "OldHorde" "EnableTeamDamage"))
  (bind (_isvalid_3 _returnvalue_3) (`MordhauUtilityLibrary.GetCustomConfigVar_Bool` "OldHorde" "EnableExplosives"))
  (bind (_isvalid_4 _returnvalue_4) (`MordhauUtilityLibrary.GetCustomConfigVar_Bool` "OldHorde" "UsePlayerScaling"))
  (bind (_isvalid_5 _returnvalue_5) (`MordhauUtilityLibrary.GetCustomConfigVar_Bool` "OldHorde" "EnableSell"))
  (`|ExecutionSequence`
    (:`then_0`
      (if _isvalid_2
        (set `self.TeamDamage` _returnvalue_2)
        (else
          (`MordhauUtilityLibrary.SetCustomConfigVar_Bool` "OldHorde" "EnableTeamDamage")
          (set `self.TeamDamage` false))))
    (:`then_1`
      (if _isvalid
        (set `self.WaveEnemySpawnOffset` _returnvalue)))
    (:`then_2`
      (if (and _isvalid_5 _returnvalue_5)
        (set `self.EnableSell` true)
        (else
          (set `self.EnableSell` false))))
    (:`then_3`
      (if (and _isvalid_3 _returnvalue_3)
        (set `self.EnableExplosives` true)
        (else
          (set `self.EnableExplosives` false))))
    (:`then_4`
      (if _isvalid_4
        (set `self.UseAdditionalPlayerScaling` _returnvalue_4)))
    (:`then_5`
      (return true))))

(fn `PrepareAIControllers`
  (for _ (range (`self.MaxAliveEnemies`))
    (bind _returnvalue (`|SpawnActorFromClass` (`self.AIControllerClass`) (`KismetMathLibrary.MakeTransform` (0.0 0.0 0.0)) "Undefined" "OverrideRootScale" null null))
    (bind _asbp_horde_aicontroller (cast `/Game/Mordhau/AI/BP_HordeAIController` _returnvalue))
    (`KismetArrayLibrary.Array_Add` (`self.AIControllers`) _asbp_horde_aicontroller)))

(fn `UserConstructionScript`
  (`parent.UserConstructionScript`))
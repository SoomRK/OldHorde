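; BP_OldHordeCharacter_Seymour is the Seymour Horde character Blueprint, which takes reduced damage from certain bosses.
; Its ModifyDamage override runs the parent calculation, then scales the result down by 15% when the instigator's controlled pawn is a Boss_Ogre or Boss1 Horde enemy.
; The construction script only calls its parent.
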(fn `ModifyDamage`
  (params (DamageAmount :type "Float (double-precision)") (DamageInfo :type "MordhauDamageInfo Structure (by ref)") (EventInstigator :type "Controller Object Reference"))
  (returns (ReturnValue :type "Float (double-precision)"))
  (locals (Temp :type "Float (double-precision)" :default 1.0))
  (bind _returnvalue (`Controller.K2_GetPawn` EventInstigator))
  (bind _returnvalue_2 (- (`local.Temp`) 0.15))
  (bind _returnvalue_3 (`parent.ModifyDamage` DamageAmount DamageInfo EventInstigator))
  (set `local.Temp` 1.0)
  (`|ExecutionSequence`
    (:`then_0`
      (cast `/Game/Mordhau/Blueprints/GameModes/Horde/BP_HordeEnemy_Boss_Ogre` _returnvalue
        (:`then`
          (set `local.Temp` _returnvalue_2))
        (:`CastFailed`
          (cast `/Game/Mordhau/Blueprints/GameModes/Horde/BP_HordeEnemy_Boss1` _returnvalue)
          (set `local.Temp` _returnvalue_2))))
    (:`then_1`
      (return (* _returnvalue_3 (`local.Temp`))))))

(fn `UserConstructionScript`
  (`parent.UserConstructionScript`))
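; BP_Ummmmm is a placeable modular character that plays the looping DancyBoi animation when play begins.
; The construction script sets UMAMaster as the master pose component for the NiceHelmet and Pants meshes, so they follow its skeleton.
; Tick is empty, and an unconnected transform-lerp node chain for a vertical offset never runs.
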(event `self.ReceiveBeginPlay`
  (`SkeletalMeshComponent.PlayAnimation` (`self.UMA_Master`) "/Game/Mordhau/Animations/RawClips/Misc/Emotes/DancyBoi.DancyBoi" true))

(event `self.ReceiveTick`
  (params (DeltaSeconds :type "Float (single-precision)")))

(fn `UserConstructionScript`
  (`SkinnedMeshComponent.SetLeaderPoseComponent` (`self.Nice_helmet`) (`self.UMA_Master`) false)
  (`SkinnedMeshComponent.SetLeaderPoseComponent` (`self.Pants`) (`self.UMA_Master`) false))
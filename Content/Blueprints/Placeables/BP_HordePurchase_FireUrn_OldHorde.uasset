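; A placeable fire urn purchase for the Old Horde game mode, extending its parent's behavior.
; One second after BeginPlay it checks the Old Horde game mode and, if explosives are disabled, turns on replication and destroys itself.
; When destroyed, it removes itself from the game state's Purchasables list before running the parent's Destroyed logic.
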(event `self.ReceiveBeginPlay`
  (`parent.ReceiveBeginPlay`)
  (`KismetSystemLibrary.Delay` 1.0)
  (bind _asbp_old_horde_game_mode (cast `/OldHorde/Blueprints/BP_OldHordeGameMode` (`GameplayStatics.GetGameMode`)))
  (if (not (`/OldHorde/Blueprints/BP_OldHordeGameMode.EnableExplosives` _asbp_old_horde_game_mode))
    (`self.SetReplicates` true)
    (`self.K2_DestroyActor`)))

(event `self.ReceiveDestroyed`
  (`|ExecutionSequence`
    (:`then_0`
      (bind _asbp_old_horde_game_state (cast `/OldHorde/Blueprints/BP_OldHordeGameState` (`GameplayStatics.GetGameState`)))
      (`KismetArrayLibrary.Array_RemoveItem` (`/Game/Mordhau/Blueprints/GameModes/Horde/BP_HordeGameState.Purchasables` _asbp_old_horde_game_state) self))
    (:`then_1`
      (`parent.ReceiveDestroyed`))))

(fn `UserConstructionScript`
  (`parent.UserConstructionScript`))
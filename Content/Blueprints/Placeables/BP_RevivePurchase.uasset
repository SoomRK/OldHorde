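; Horde-mode purchasable, shown as a player grave, that charges coins at the game state's revive cost to call HealTeam on the game mode.
; CanInteract checks the player's coins, and OnInteractionStart deducts the cost.
; UpdateVisuals lazily builds the mesh and widget, syncs cost and local affordability, and toggles widget visibility by camera distance with hysteresis.
; On destruction it removes itself from the game state's Purchasables.
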(event `self.ReceiveBeginPlay`
  (`parent.ReceiveBeginPlay`)
  (`KismetSystemLibrary.Delay` 0.5)
  (bind _asbp_old_horde_game_state (cast `/OldHorde/Blueprints/BP_OldHordeGameState` (`GameplayStatics.GetGameState`)))
  (set `self.Cost` (`/OldHorde/Blueprints/BP_OldHordeGameState.ReviveCost` _asbp_old_horde_game_state)))

(event `self.OnInteractionStart`
  (params (Character :type "MordhauCharacter Object Reference"))
  (`/Engine/EditorBlueprintResources/StandardMacros.IsValid` Character
    (:`Is Valid`
      (bind _asbp_horde_character (cast `/Game/Mordhau/Blueprints/Characters/BP_HordeCharacter` Character))
      (bind _asbp_horde_player_state (cast `/Game/Mordhau/Blueprints/GameModes/Horde/BP_HordePlayerState` (`Pawn.PlayerState` Character)))
      (set `/Game/Mordhau/Blueprints/GameModes/Horde/BP_HordePlayerState.Coins` (- (`/Game/Mordhau/Blueprints/GameModes/Horde/BP_HordePlayerState.Coins` _asbp_horde_player_state) (`self.Cost`)) _asbp_horde_player_state)
      (bind _asbp_old_horde_game_mode (cast `/OldHorde/Blueprints/BP_OldHordeGameMode` (`GameplayStatics.GetGameMode`)))
      (`/OldHorde/Blueprints/BP_OldHordeGameMode.HealTeam` _asbp_old_horde_game_mode _asbp_horde_character))))

(event `self.ReceiveDestroyed`
  (`|ExecutionSequence`
    (:`then_0`
      (bind _asbp_old_horde_game_state (cast `/OldHorde/Blueprints/BP_OldHordeGameState` (`GameplayStatics.GetGameState`)))
      (`KismetArrayLibrary.Array_RemoveItem` (`/Game/Mordhau/Blueprints/GameModes/Horde/BP_HordeGameState.Purchasables` _asbp_old_horde_game_state) self))
    (:`then_1`
      (`parent.ReceiveDestroyed`))))

(fn `CanInteract`
  (params (Character :type "MordhauCharacter Object Reference"))
  (returns (ReturnValue :type Boolean))
  (`/Engine/EditorBlueprintResources/StandardMacros.IsValid` Character
    (:`Is Valid`
      (bind _asbp_horde_player_state (cast `/Game/Mordhau/Blueprints/GameModes/Horde/BP_HordePlayerState` (`Pawn.PlayerState` Character)))
      (if (>= (`/Game/Mordhau/Blueprints/GameModes/Horde/BP_HordePlayerState.Coins` _asbp_horde_player_state) (`self.Cost`))
        (return true)
        (else
          (return false))))))

(fn `InitializeDisplay`
  (`SkinnedMeshComponent.SetSkinnedAssetAndUpdate` (`self.LODSkeletalMesh`) null true)
  (`StaticMeshComponent.SetStaticMesh` (`self.StaticMesh`) "/Game/Mordhau/Assets/Interactables/Mesh/Horde_PlayerGrave/SM_Horde_PlayerGrave.SM_Horde_PlayerGrave")
  (`|ExecutionSequence`
    (:`then_0`
      (bind _returnvalue (`MordhauUtilityLibrary.GetComponentsBoundingBoxInActorSpace` self))
      (bind _returnvalue_2 (`AddComponent|NODE_AddMordhauWidgetComponent-0` :`RelativeTransform` (`KismetMathLibrary.MakeTransform` _returnvalue)))
      (set `self.Widget` _returnvalue_2))
    (:`then_1`
      (bind _asbp_old_horde_game_state (cast `/OldHorde/Blueprints/BP_OldHordeGameState` (`GameplayStatics.GetGameState`)))
      (set `self.Cost` (`/OldHorde/Blueprints/BP_OldHordeGameState.ReviveCost` _asbp_old_horde_game_state)))
    (:`then_2`
      (`self.SetAvailability` false)
      (set `self.Initialized` true))))

(fn `UpdateVisuals`
  (bind _returnvalue (`GameplayStatics.GetPlayerController` 0))
  (bind _isavailable (`self.IsAvailable`))
  (bind _returnvalue_2 (`KismetMathLibrary.VSize` (- (`self.K2_GetActorLocation`) (`PlayerCameraManager.GetCameraLocation` (`GameplayStatics.GetPlayerCameraManager` 0)))))
  (`|ExecutionSequence`
    (:`then_0`
      (if (not (`self.Initialized`))
        (`self.InitializeDisplay`)))
    (:`then_1`
      (`/Engine/EditorBlueprintResources/StandardMacros.IsValid` _returnvalue
        (:`Is Valid`
          (if (`Controller.IsLocalPlayerController` _returnvalue)
            (`|ExecutionSequence`
              (:`then_0`
                (bind _asbp_old_horde_game_state (cast `/OldHorde/Blueprints/BP_OldHordeGameState` (`GameplayStatics.GetGameState`)))
                (bind _revivecost (`/OldHorde/Blueprints/BP_OldHordeGameState.ReviveCost` _asbp_old_horde_game_state))
                (if (not (== _revivecost (`self.Cost`)))
                  (set `self.Cost` _revivecost)))
              (:`then_1`
                (bind _asbp_horde_player_state (cast `/Game/Mordhau/Blueprints/GameModes/Horde/BP_HordePlayerState` (`Controller.PlayerState` _returnvalue)))
                (if (not (== _isavailable (>= (`/Game/Mordhau/Blueprints/GameModes/Horde/BP_HordePlayerState.Coins` _asbp_horde_player_state) (`self.Cost`))))
                  (`self.SetAvailability` (not _isavailable))))
              (:`then_2`
                (`|ExecutionSequence`
                  (:`then_0`
                    (set `self.IsValid` true))
                  (:`then_1`
                    (if (!= (`MordhauWidgetComponent.OverrideVisible` (`self.Widget`)) 0)
                      (if (not (< _returnvalue_2 (+ 600.0 25.0)))
                        (set `MordhauWidgetComponent.OverrideVisible` 0 (`self.Widget`)))
                      (elif (< _returnvalue_2 600.0)
                        (set `MordhauWidgetComponent.OverrideVisible` -1 (`self.Widget`))))))))))))))

(fn `UserConstructionScript`
  (`parent.UserConstructionScript`))
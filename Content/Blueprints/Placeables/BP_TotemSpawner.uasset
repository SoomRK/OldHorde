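; BP_TotemSpawner is a placeable that spawns a gold totem at its capsule's location and respawns it after pickup.
; On BeginPlay it spawns the first totem with authority only, passing it a spawner reference, coin amount and display text.
; Its PickedUpTotem dispatcher triggers RespawnTimer, which destroys any current totem, waits a configurable delay, then attempts the authority-gated spawn again.
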(event `RespawnTimer`
  (bind _currenttotem (`self.CurrentTotem`))
  (`/Engine/EditorBlueprintResources/StandardMacros.IsValid` _currenttotem
    (:`Is Valid`
      (`self.K2_DestroyActor` _currenttotem))
    (:`Is Not Valid`
      _))
  (`KismetSystemLibrary.Delay` (`self.Time`))
  (`self.TrySpawnTotem`))

(event `self.ReceiveBeginPlay`
  (`parent.ReceiveBeginPlay`)
  (`self.TrySpawnTotem`)
  (add `self.PickedUpTotem` (delegate `RespawnTimer`)))

(event `SpawnTotem`
  (bind _returnvalue (`|SpawnActorFromClass` "/OldHorde/Blueprints/Placeables/BP_GoldTotem.BP_GoldTotem_C" (`KismetMathLibrary.MakeTransform` (`SceneComponent.K2_GetComponentLocation` (`self.Capsule`)) (`self.K2_GetActorRotation`)) "AlwaysSpawn" "OverrideRootScale" null null))
  (set `/OldHorde/Blueprints/Placeables/BP_GoldTotem.TotemSpawner` self _returnvalue)
  (set `self.CurrentTotem` _returnvalue)
  (set `/OldHorde/Blueprints/Placeables/BP_GoldTotem.CoinsToAdd` (`self.Coins to Add`) _returnvalue)
  (set `/OldHorde/Blueprints/Placeables/BP_GoldTotem.Display Text` (`self.Display Text`) _returnvalue))

(fn `TrySpawnTotem`
  (`/Engine/EditorBlueprintResources/ActorMacros.Switch Has Authority`
    (:`Authority`
      (`self.SpawnTotem`))))

(fn `UserConstructionScript`
  (`parent.UserConstructionScript`))
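; Tier 2 Horde chest variant that sells a random item to players with enough coins.
; Interaction deducts the cost, runs SpawnItem, increments the controller's PurchaseTrigger, then breaks the chest by disabling collision and flagging it destroyed.
; Spawned equipment gets the player's emblem and default customization (random as fallback), restocks matching gear, then is equipped or left to ragdoll.
; Wearable pickups equip only if they are an upgrade.
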(event `self.OnInteractionStart`
  (params (Character :type "MordhauCharacter Object Reference"))
  (bind _cost (`self.Cost`))
  (`/Engine/EditorBlueprintResources/StandardMacros.IsValid` Character
    (:`Is Valid`
      (bind _asbp_horde_player_state (cast `/Game/Mordhau/Blueprints/GameModes/Horde/BP_HordePlayerState` (`Pawn.PlayerState` Character)))
      (cast `/Game/Mordhau/Blueprints/GameModes/Horde/BP_HordePlayerController` (`self.GetOwner` _asbp_horde_player_state))
      (bind _coins (`/Game/Mordhau/Blueprints/GameModes/Horde/BP_HordePlayerState.Coins` _asbp_horde_player_state))
      (if (>= _coins _cost)
        (set `/Game/Mordhau/Blueprints/GameModes/Horde/BP_HordePlayerState.Coins` (- _coins _cost) _asbp_horde_player_state)
        (bind _asbp_battle_royale_character (cast `/Game/Mordhau/Blueprints/Characters/BP_BattleRoyaleCharacter` Character))
        (`|ExecutionSequence`
          (:`then_0`
            (`self.SpawnItem` _asbp_battle_royale_character))
          (:`then_1`
            (bind _asbp_horde_player_controller (cast `/Game/Mordhau/Blueprints/GameModes/Horde/BP_HordePlayerController` (`Pawn.GetController` _asbp_battle_royale_character)))
            (set `/Game/Mordhau/Blueprints/GameModes/Horde/BP_HordePlayerController.PurchaseTrigger` (+ (`/Game/Mordhau/Blueprints/GameModes/Horde/BP_HordePlayerController.PurchaseTrigger` _asbp_horde_player_controller) 1) _asbp_horde_player_controller))
          (:`then_2`
            (`self.BreakChest` null)))))))

(fn `BreakChest`
  (params (DestroyerPlayerController :type "MordhauPlayerController Object Reference"))
  (if (not (`self.ChestDestroyed`))
    (`PrimitiveComponent.SetCollisionEnabled` (`self.SkeletalMesh`) "NoCollision")
    (set `self.ChestDestroyed` true)))

(fn `CanInteract`
  (params (Character :type "MordhauCharacter Object Reference"))
  (returns (ReturnValue :type Boolean))
  (`/Engine/EditorBlueprintResources/StandardMacros.IsValid` Character
    (:`Is Valid`
      (bind _asbp_horde_player_state (cast `/Game/Mordhau/Blueprints/GameModes/Horde/BP_HordePlayerState` (`Pawn.PlayerState` Character)))
      (return (>= (`/Game/Mordhau/Blueprints/GameModes/Horde/BP_HordePlayerState.Coins` _asbp_horde_player_state) (`self.Cost`))))))

(fn `SpawnItem`
  (params (ForCharacter :type "/Game/Mordhau/Blueprints/Characters/BP_BattleRoyaleCharacter Object Reference"))
  (locals (Emblem :type Integer) (EmblemColor1 :type Byte) (EmblemColor2 :type Byte) (Customization :type "EquipmentCustomization Structure"))
  (bind _founditem (`self.GetRandomItem`))
  (bind _returnvalue (`|SpawnActorFromClass` _founditem (`self.GetTransform`) "Undefined" "OverrideRootScale" null null))
  (bind _asmordhau_equipment (cast `MordhauEquipment` _returnvalue)
    (:`then`
      (bind _returnvalue_2 (`MordhauEquipment.GetRandomCustomization` _asmordhau_equipment true))
      (set `local.Customization` _returnvalue_2)
      (`|ExecutionSequence`
        (:`then_0`
          (bind _asmordhau_player_controller (cast `MordhauPlayerController` (`Pawn.GetController` ForCharacter)))
          (bind (_emblem _emblemcolors) (break `AppearanceCustomization` (`.AppearanceCustomization` (break `CharacterProfile` (`MordhauPlayerController.CharacterProfile` _asmordhau_player_controller)))))
          (set `local.Emblem` _emblem)
          (set `local.EmblemColor1` (`|GetArrayItem` _emblemcolors))
          (set `local.EmblemColor2` (`|GetArrayItem` _emblemcolors 1))
          (bind (_outcustomization _returnvalue_3) (`MordhauPlayerController.GetDefaultEquipmentCustomizationFor` _asmordhau_player_controller (`GameplayStatics.GetObjectClass` _asmordhau_equipment)))
          (if _returnvalue_3
            (set `local.Customization` _outcustomization)))
        (:`then_1`
          (`MordhauEquipment.AssignCustomization` _asmordhau_equipment (`local.Customization`) (`KismetMathLibrary.Conv_IntToByte` (`local.Emblem`)) (`local.EmblemColor1`) (`local.EmblemColor2`))
          (`MordhauEquipment.RestockOtherEquipmentOnCharacter` _asmordhau_equipment ForCharacter)
          (if (not (and (`MordhauEquipment.bDestroyIfNoAmmo` _asmordhau_equipment) (== (`MordhauEquipment.GetAmmo` _asmordhau_equipment) 0)))
            (bind _returnvalue_4 (`MordhauCharacter.PickUp` ForCharacter _asmordhau_equipment -1))
            (if _returnvalue_4
              (`MordhauCharacter.SwitchEquipment` ForCharacter _asmordhau_equipment)
              (else
                (set `MordhauEquipment.bCanRagdoll` true _asmordhau_equipment)
                (`MordhauEquipment.UpdateEquipmentState` _asmordhau_equipment)))))))
    (:`CastFailed`
      (bind _asbp_wearable_pickup (cast `/Game/Mordhau/Blueprints/Interactables/WearablePickups/BP_WearablePickup` _returnvalue))
      (`/Game/Mordhau/Blueprints/Interactables/WearablePickups/BP_WearablePickup.EquipIfUpgrade` _asbp_wearable_pickup ForCharacter))))

(fn `UserConstructionScript`
  (`parent.UserConstructionScript`))
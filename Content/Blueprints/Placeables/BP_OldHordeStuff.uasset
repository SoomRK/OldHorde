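; Placeable Horde-mode helper that unsticks idle enemies and adds admin chat commands, destroying itself unless the OldHorde EnableCommands config is on.
; A server timer clears the perceived-enemy blackboard key on idle or motionless living enemies, damaging those without controllers.
; The game mode's message broadcast feeds string-parsing helpers for granting coins to oneself, a named player or everyone, and killing the wave.
; Skill-point command branches exist but are disconnected.
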(event `self.ReceiveBeginPlay`
  (`parent.ReceiveBeginPlay`)
  (`/Engine/EditorBlueprintResources/ActorMacros.Switch Has Authority`
    (:`Authority`
      (`KismetSystemLibrary.K2_SetTimerDelegate` (delegate `TimerHordeIdleCheck`) 5.0 true))))

(event `TimerHordeIdleCheck`
  (bind _outactors (`GameplayStatics.GetAllActorsOfClass` "/Game/Mordhau/Blueprints/GameModes/Horde/BP_HordeEnemy.BP_HordeEnemy_C"))
  (if (> (`KismetArrayLibrary.Array_Length` _outactors) 0)
    (for _array_element _outactors
      (`/Engine/EditorBlueprintResources/StandardMacros.IsValid` _array_element
        (:`Is Valid`
          (if (not (`AdvancedCharacter.GetIsDead` _array_element))
            (bind _returnvalue (`AdvancedCharacter.GetMotion` _array_element))
            (`/Engine/EditorBlueprintResources/StandardMacros.IsValid` _returnvalue
              (:`Is Valid`
                (cast `IdleMotion` _returnvalue))
              (:`Is Not Valid`
                _))
            (bind _returnvalue_2 (`AdvancedCharacter.GetControllerIncludingVehicle` _array_element))
            (`/Engine/EditorBlueprintResources/StandardMacros.IsValid` _returnvalue_2
              (:`Is Valid`
                (bind _asbp_horde_aicontroller (cast `/Game/Mordhau/AI/BP_HordeAIController` _returnvalue_2))
                (`BlackboardComponent.ClearValue` (`AIBlueprintHelperLibrary.GetBlackboard` _asbp_horde_aicontroller) "bPerceivesEnemy"))
              (:`Is Not Valid`
                (`AdvancedCharacter.MordhauTakeDamage` _array_element 50.0 (`GameplayStatics.MakeHitResult` false) "Generic" 0 null null null)))))))))

(event `self.ReceiveTick`
  (params (DeltaSeconds :type "Float (single-precision)"))
  (bind _returnvalue (`GameplayStatics.GetGameMode`))
  (`parent.ReceiveTick` DeltaSeconds)
  (`/Engine/EditorBlueprintResources/StandardMacros.IsValid` _returnvalue
    (:`Is Valid`
      (`/Engine/EditorBlueprintResources/StandardMacros.DoOnce` false
        (:`Completed`
          (if (`self.GetConfig`)
            (bind _asbp_mordhau_game_mode (cast `/Game/Mordhau/Blueprints/GameModes/BP_MordhauGameMode` _returnvalue))
            (add `MordhauGameMode.OnMessageBroadcasted` _asbp_mordhau_game_mode (delegate `CustomEvent_0`))
            (else
              (`self.K2_DestroyActor`))))))))

(event `CustomEvent_0`
  (params (Sender :type "Actor Object Reference") (Msg :type String) (Type :type Name))
  (bind (_returnvalue _returnvalue1) (`self.MessageHasCommand` Msg ".coinsall "))
  (bind (_returnvalue_2 _returnvalue1_2) (`self.MessageHasCommand` Msg ".coins "))
  (bind (_playername _value _newparam) (`self.ParseMessage` _returnvalue1_2))
  (bind _returnvalue_3 (> _value 0))
  (bind _asbp_horde_player_controller (cast `/Game/Mordhau/Blueprints/GameModes/Horde/BP_HordePlayerController` Sender))
  (if (`MordhauPlayerController.IsAdmin` _asbp_horde_player_controller)
    (if _returnvalue_2
      (if (and (`KismetStringLibrary.EqualEqual_StrStr` _playername "invalid") _returnvalue_3)
        (bind _asbp_horde_player_state (cast `/Game/Mordhau/Blueprints/GameModes/Horde/BP_HordePlayerState` (`Controller.PlayerState` _asbp_horde_player_controller)))
        (set `/Game/Mordhau/Blueprints/GameModes/Horde/BP_HordePlayerState.Coins` (+ (`/Game/Mordhau/Blueprints/GameModes/Horde/BP_HordePlayerState.Coins` _asbp_horde_player_state) _value) _asbp_horde_player_state)
        (elif (and _returnvalue_3 (not (== _newparam null)))
          (bind _asbp_horde_player_state_2 (cast `/Game/Mordhau/Blueprints/GameModes/Horde/BP_HordePlayerState` _newparam))
          (set `/Game/Mordhau/Blueprints/GameModes/Horde/BP_HordePlayerState.Coins` (+ (`/Game/Mordhau/Blueprints/GameModes/Horde/BP_HordePlayerState.Coins` _asbp_horde_player_state_2) _value) _asbp_horde_player_state_2)))
      (elif (`self.MessageHasCommand` Msg ".endwave")
        (bind _outactors (`GameplayStatics.GetAllActorsOfClass` "/Game/Mordhau/Blueprints/GameModes/Horde/BP_HordeEnemy.BP_HordeEnemy_C"))
        (if (> (`KismetArrayLibrary.Array_Length` _outactors) 0)
          (for _array_element _outactors
            (`AdvancedCharacter.MordhauTakeDamage` _array_element 6969.0 (`GameplayStatics.MakeHitResult` false) "Generic" 0 null null _asbp_horde_player_controller)))
        (elif _returnvalue
          (bind _outactors_2 (`GameplayStatics.GetAllActorsOfClass` "/Game/Mordhau/Blueprints/GameModes/Horde/BP_HordePlayerState.BP_HordePlayerState_C"))
          (if (> (`KismetArrayLibrary.Array_Length` _outactors_2) 0)
            (for _array_element_2 _outactors_2
              (`/Engine/EditorBlueprintResources/StandardMacros.IsValid` _array_element_2
                (:`Is Valid`
                  (set `/Game/Mordhau/Blueprints/GameModes/Horde/BP_HordePlayerState.Coins` (+ (`/Game/Mordhau/Blueprints/GameModes/Horde/BP_HordePlayerState.Coins` _array_element_2) (`.Value` (`self.ParseMessage` _returnvalue1))) _array_element_2))))))))))

(fn `GetConfig`
  (returns (ReturnValue :type Boolean))
  (bind (_isvalid _returnvalue) (`MordhauUtilityLibrary.GetCustomConfigVar_Bool` "OldHorde" "EnableCommands"))
  (if _isvalid
    (return _returnvalue)))

(fn `GetPlayer`
  (params (Player :type String))
  (returns (`Array Element` :type "PlayerState Object Reference") (ReturnValue :type Boolean))
  (bind _asbp_horde_game_state (cast `/Game/Mordhau/Blueprints/GameModes/Horde/BP_HordeGameState` (`GameplayStatics.GetGameState`)))
  (for _array_element (`GameStateBase.PlayerArray` _asbp_horde_game_state)
    (if (`KismetStringLibrary.Contains` (`PlayerState.GetPlayerName` _array_element) Player)
      (return _array_element true)))
  (return null false))

(fn `MessageHasCommand`
  (params (Message :type String) (Command :type String))
  (returns (ReturnValue :type Boolean) (ReturnValue1 :type String))
  (locals (MessageX :type String) (CommandX :type String))
  (bind _messagex (`local.MessageX`))
  (bind _returnvalue (`KismetStringLibrary.Len` (`local.CommandX`)))
  (set `local.MessageX` Message)
  (set `local.CommandX` Command)
  (if (`KismetStringLibrary.StartsWith` _messagex (`local.CommandX`))
    (return true (`KismetStringLibrary.GetSubstring` _messagex _returnvalue (- (`KismetStringLibrary.Len` (`local.MessageX`)) _returnvalue)))
    (else
      (return false ""))))

(fn `ParseMessage`
  (params (Message :type String))
  (returns (PlayerName :type String) (Value :type Integer) (NewParam :type "PlayerState Object Reference"))
  (locals (Temp :type String))
  (bind _output_get (set `local.Temp` Message))
  (if (`KismetStringLibrary.Contains` _output_get " ")
    (bind (_lefts _rights) (`KismetStringLibrary.Split` _output_get " "))
    (if (`KismetStringLibrary.EqualEqual_StrStr` _rights)
      _
      (else
        (bind (_array_element _returnvalue) (`self.GetPlayer` _lefts))
        (if _returnvalue
          (return _lefts (`KismetStringLibrary.Conv_StringToInt` _rights) _array_element)
          (else
            (return "invalid" 0 null))))))
  (return "invalid" (`KismetStringLibrary.Conv_StringToInt` _output_get) null))

(fn `StripChars`
  (params (String :type String) (CharsToStrip :type String))
  (returns (ReturnValue :type String))
  (locals (StringChars :type "Array of String") (StripCharacters :type "Array of String") (ResultString :type String) (AllExcept :type Boolean))
  (set `local.StringChars` (`KismetStringLibrary.GetCharacterArrayFromString` String))
  (set `local.StripCharacters` (`KismetStringLibrary.GetCharacterArrayFromString` CharsToStrip))
  (for _array_element (`local.StringChars`)
    (if (`local.AllExcept`)
      (bind _returnvalue (`KismetArrayLibrary.Array_Contains` (`local.StripCharacters`) _array_element))
      (if (not (not _returnvalue))
        (set `local.ResultString` (`KismetStringLibrary.Concat_StrStr` (`local.ResultString`) _array_element) :!label _label))
      (elif (not _returnvalue)
        (goto _label))))
  (return (`local.ResultString`)))

(fn `UserConstructionScript`
  (`parent.UserConstructionScript`))
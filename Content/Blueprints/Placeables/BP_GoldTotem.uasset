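; BP_GoldTotem is a Horde mode pickup that grants coins and a gold bonus to the player who interacts with it.
; Only Horde characters can interact, which adds coins to player state and increments the controller's GoldBonus.
; It then leaves the game state's Purchasables, notifies any TotemSpawner and destroys itself.
; Visual updates lazily create the mesh and widget, toggling widget visibility by camera distance with hysteresis.
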(event `self.OnInteractionStart`
  (params (Character :type "MordhauCharacter Object Reference"))
  (bind _totemspawner (`self.TotemSpawner`))
  (bind _asbp_horde_player_state (cast `/Game/Mordhau/Blueprints/GameModes/Horde/BP_HordePlayerState` (`Pawn.PlayerState` Character)))
  (set `/Game/Mordhau/Blueprints/GameModes/Horde/BP_HordePlayerState.Coins` (+ (`/Game/Mordhau/Blueprints/GameModes/Horde/BP_HordePlayerState.Coins` _asbp_horde_player_state) (`self.CoinsToAdd`)) _asbp_horde_player_state)
  (`|ExecutionSequence`
    (:`then_0`
      (bind _asbp_old_horde_player_controller (cast `/OldHorde/Blueprints/BP_OldHordePlayerController` (`AdvancedCharacter.GetControllerIncludingVehicle` Character)))
      (set `/OldHorde/Blueprints/BP_OldHordePlayerController.GoldBonus` (+ (`/OldHorde/Blueprints/BP_OldHordePlayerController.GoldBonus` _asbp_old_horde_player_controller) 1) _asbp_old_horde_player_controller))
    (:`then_1`
      (bind _asbp_horde_game_state (cast `/Game/Mordhau/Blueprints/GameModes/Horde/BP_HordeGameState` (`GameplayStatics.GetGameState`)))
      (bind _purchasables (`/Game/Mordhau/Blueprints/GameModes/Horde/BP_HordeGameState.Purchasables` _asbp_horde_game_state))
      (bind _returnvalue (`KismetArrayLibrary.Array_Find` _purchasables self))
      (if (not (== _returnvalue -1))
        (`KismetArrayLibrary.Array_Remove` _purchasables _returnvalue)
        (set `/Game/Mordhau/Blueprints/GameModes/Horde/BP_HordeGameState.Purchasables` _purchasables _asbp_horde_game_state)))
    (:`then_2`
      (if (== _totemspawner null)
        (`self.SetReplicates` true)
        (`self.K2_DestroyActor`)
        (else
          (`/OldHorde/Blueprints/Placeables/BP_TotemSpawner.PickedUpTotem` _totemspawner)
          (`self.SetReplicates` true)
          (`self.K2_DestroyActor`))))))

(fn `CanInteract`
  (params (Character :type "MordhauCharacter Object Reference"))
  (returns (ReturnValue :type Boolean))
  (`/Engine/EditorBlueprintResources/StandardMacros.IsValid` Character
    (:`Is Valid`
      (cast `/Game/Mordhau/Blueprints/Characters/BP_HordeCharacter` Character
        (:`then`
          (return true))
        (:`CastFailed`
          _)))
    (:`Is Not Valid`
      _))
  (return false))

(fn `InitializeDisplay`
  (`|ExecutionSequence`
    (:`then_0`
      (`SkinnedMeshComponent.SetSkinnedAssetAndUpdate` (`self.LODSkeletalMesh`) null true)
      (`StaticMeshComponent.SetStaticMesh` (`self.StaticMesh`) (`self.New Mesh`)))
    (:`then_1`
      (bind _returnvalue (`MordhauUtilityLibrary.GetComponentsBoundingBoxInActorSpace` self))
      (bind _returnvalue_2 (`AddComponent|NODE_AddMordhauWidgetComponent-0` :`RelativeTransform` (`KismetMathLibrary.MakeTransform` _returnvalue)))
      (set `self.Widget` _returnvalue_2))
    (:`then_2`
      (`self.SetAvailability` false)
      (set `self.Initialized` true))))

(fn `UpdateVisuals`
  (bind _returnvalue (`GameplayStatics.GetPlayerController` 0))
  (bind _returnvalue_2 (`KismetMathLibrary.VSize` (- (`self.K2_GetActorLocation`) (`PlayerCameraManager.GetCameraLocation` (`GameplayStatics.GetPlayerCameraManager` 0)))))
  (`|ExecutionSequence`
    (:`then_0`
      (if (not (`self.Initialized`))
        (`self.InitializeDisplay`)))
    (:`then_1`
      (`/Engine/EditorBlueprintResources/StandardMacros.IsValid` _returnvalue
        (:`Is Valid`
          (if (`Controller.IsLocalPlayerController` _returnvalue)
            (`|ExecutionSequence`
              (:`then_0`
                (set `self.IsValid` true))
              (:`then_1`
                (if (!= (`MordhauWidgetComponent.OverrideVisible` (`self.Widget`)) 0)
                  (if (not (< _returnvalue_2 (+ 200.0 25.0)))
                    (set `MordhauWidgetComponent.OverrideVisible` 0 (`self.Widget`)))
                  (elif (< _returnvalue_2 200.0)
                    (set `MordhauWidgetComponent.OverrideVisible` -1 (`self.Widget`))))))))))))

(fn `UserConstructionScript`
  (`parent.UserConstructionScript`))
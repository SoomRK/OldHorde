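; HUD for the Old Horde mode that owns the horde HUD, gold gift and skill tree widgets.
; It creates them once game state replicates, passing the skill tree setting to HUD and gifts, and shows the "Slay the Horde!" objective.
; HUD visibility follows minimal/full mode and main menu events, and match results remove it.
; Tick polls replicated match info to re-announce the objective when a new wave has spawned enemies.
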(event `self.ReceiveBeginPlay`
  (`parent.ReceiveBeginPlay`))

(event `self.OnGameStateReplicated`
  (bind _returnvalue (`GameplayStatics.GetPlayerController` 0))
  (`parent.OnGameStateReplicated`)
  (bind _asbp_old_horde_game_state (cast `/OldHorde/Blueprints/BP_OldHordeGameState` (`GameplayStatics.GetGameState`)))
  (`|ExecutionSequence`
    (:`then_0`
      (`/Engine/EditorBlueprintResources/StandardMacros.IsValid` _returnvalue
        (:`Is Valid`
          (bind _useskilltree (`/OldHorde/Blueprints/BP_OldHordeGameState.UseSkillTree` _asbp_old_horde_game_state))
          (bind _returnvalue_2 (`|CreateWidget` "/OldHorde/Blueprints/BP_OldHordeHUDWidget_Seymour.BP_OldHordeHUDWidget_Seymour_C" _returnvalue _useskilltree))
          (bind _output_get (set `self.HordeHUDWidget` _returnvalue_2))
          (`UserWidget.AddToViewport` _output_get -5)
          (if (`self.IsHUDMinimal`)
            (`Widget.SetVisibility` _output_get "Collapsed")))))
    (:`then_1`
      (`self.MakeGoldGifts` _useskilltree)
      (`self.CreateSkillTree`)
      (bind _asbp_mordhau_hud (cast `/Game/Mordhau/Blueprints/BP_MordhauHUD` (`PlayerController.GetHUD` (`GameplayStatics.GetPlayerController` 0))))
      (`self.ShowObjectiveWidget` _asbp_mordhau_hud "Slay the Horde!" "Objective:" null))))

(event `self.UseMinimalHUD`
  (`parent.UseMinimalHUD`)
  (`/Engine/EditorBlueprintResources/StandardMacros.IsValid` (`self.HordeHUDWidget`)
    (:`Is Valid`
      (`Widget.SetVisibility` (`self.HordeHUDWidget`) "Collapsed"))))

(event `self.UseFullHUD`
  (`parent.UseFullHUD`)
  (`/Engine/EditorBlueprintResources/StandardMacros.IsValid` (`self.HordeHUDWidget`)
    (:`Is Valid`
      (`Widget.SetVisibility` (`self.HordeHUDWidget`) "Visible"))))

(event `self.HideMainMenu`
  (`parent.HideMainMenu`)
  (`Widget.SetVisibility` (`self.HordeHUDWidget`) "Visible"))

(event `self.Show Main Menu`
  (`parent.Show Main Menu`)
  (`Widget.SetVisibility` (`self.HordeHUDWidget`) "Collapsed"))

(event `self.ReceiveTick`
  (params (DeltaSeconds :type "Float (single-precision)"))
  (`parent.ReceiveTick` DeltaSeconds)
  (`self.Show Objective at RoundStart`))

(fn `CreateSkillTree`
  (bind _returnvalue (`|CreateWidget` "/OldHorde/Blueprints/BP_OldHordeSkillTree.BP_OldHordeSkillTree_C" (`GameplayStatics.GetPlayerController` 0)))
  (bind _output_get (set `self.SeymourSkills` _returnvalue))
  (`Widget.SetVisibility` _output_get "Collapsed")
  (`UserWidget.AddToViewport` _output_get 0))

(fn `MakeGoldGifts`
  (params (Skills :type Boolean))
  (bind _returnvalue (`|CreateWidget` "/OldHorde/Blueprints/BP_SeymourGiftWidget.BP_SeymourGiftWidget_C" (`GameplayStatics.GetPlayerController` 0) Skills))
  (bind _output_get (set `self.GiftWidget` _returnvalue))
  (`UserWidget.AddToViewport` _output_get 2)
  (`Widget.SetVisibility` _output_get "Collapsed"))

(fn `Show Objective at RoundStart`
  (bind _asbp_horde_game_state (cast `/Game/Mordhau/Blueprints/GameModes/Horde/BP_HordeGameState` (`GameplayStatics.GetGameState`)))
  (bind (_wave _enemiesremaining _nextwavestarttime _spawnedenemies) (break `/Game/Mordhau/Blueprints/GameModes/Horde/STRUCT_HordeMatchInfo` (`/Game/Mordhau/Blueprints/GameModes/Horde/BP_HordeGameState.ReplicatedHordeMatchInfo` _asbp_horde_game_state)))
  (if (and (!= _wave (`self.Current Wave`)) (!= _wave 255) (!= _spawnedenemies 0))
    (set `self.Current Wave` _wave)
    (bind _asbp_mordhau_hud (cast `/Game/Mordhau/Blueprints/BP_MordhauHUD` (`PlayerController.GetHUD` (`GameplayStatics.GetPlayerController` 0))))
    (`self.ShowAnnouncement` _asbp_mordhau_hud "Objective:" "Slay the Horde!" 5.0 "NewEnumerator1")))

(fn `ShowGoldGifts`
  (`/OldHorde/Blueprints/BP_SeymourGiftWidget.Show` (`self.GiftWidget`)))

(fn `ShowMatchResult`
  (params (IsVictory :type Boolean) (MainText :type Text) (SubText :type Text))
  (`parent.ShowMatchResult` IsVictory MainText SubText)
  (`Widget.RemoveFromParent` (`self.HordeHUDWidget`)))

(fn `ShowSkillTree`
  (bind _seymourskills (`self.SeymourSkills`))
  (`/Engine/EditorBlueprintResources/StandardMacros.IsValid` _seymourskills
    (:`Is Valid`
      (`/OldHorde/Blueprints/BP_OldHordeSkillTree.Show` _seymourskills))))

(fn `UserConstructionScript`
  (`parent.UserConstructionScript`))
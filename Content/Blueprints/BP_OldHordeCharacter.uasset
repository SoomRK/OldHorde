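; Horde-mode character variant that forces two perks and adjusts combat damage, with empty skill-application functions.
; On BeginPlay it polls for the customization replication actor, then on authority toggles missing perks through a temporary profile wrapper and reassigns the profile.
; It scales parent-modified damage up and boosts player bow and crossbow damage.
; It saves equipment classes and ammo to the Horde PlayerState, blanking invalid and last slots.
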(event `self.ReceiveBeginPlay`
  (`parent.ReceiveBeginPlay`)
  (`|ExecutionSequence`
    (:`then_0`
      (`KismetSystemLibrary.Delay` 0.2 :!label _label)
      (bind _returnvalue (`self.GetCustomizationReplicationActor`))
      (`/Engine/EditorBlueprintResources/StandardMacros.IsValid` _returnvalue
        (:`Is Valid`
          (if (`self.HasAuthority` _returnvalue)
            (if (not (`self.HasPerk` 8))
              (bind _returnvalue_2 (`|GenericCreateObject` "/Script/Mordhau.CharacterProfileBPWrapper" self))
              (bind _output_get (set `CharacterProfileBPWrapper.Profile` (`CustomizationReplicationActor.LastAssignedProfile` _returnvalue) _returnvalue_2))
              (`CharacterProfileBPWrapper.TogglePerk` _returnvalue_2 8)
              (`CustomizationReplicationActor.AssignDataFromProfile` _returnvalue _output_get))))
        (:`Is Not Valid`
          (goto _label))))
    (:`then_1`
      (`KismetSystemLibrary.Delay` 0.2 :!label _label_2)
      (bind _returnvalue_3 (`self.GetCustomizationReplicationActor`))
      (`/Engine/EditorBlueprintResources/StandardMacros.IsValid` _returnvalue_3
        (:`Is Valid`
          (if (`self.HasAuthority` _returnvalue_3)
            (if (not (`self.HasPerk` 15))
              (bind _returnvalue_4 (`|GenericCreateObject` "/Script/Mordhau.CharacterProfileBPWrapper" self))
              (bind _output_get_2 (set `CharacterProfileBPWrapper.Profile` (`CustomizationReplicationActor.LastAssignedProfile` _returnvalue_3) _returnvalue_4))
              (`CharacterProfileBPWrapper.TogglePerk` _returnvalue_4 15)
              (`CustomizationReplicationActor.AssignDataFromProfile` _returnvalue_3 _output_get_2))))
        (:`Is Not Valid`
          (goto _label_2))))))

(fn `ApplySkills`)

(fn `ApplySkillsToEquipment`
  (params (Equip :type "MordhauEquipment Object Reference")))

(fn `ModifyDamage`
  (params (DamageAmount :type "Float (double-precision)") (DamageInfo :type "MordhauDamageInfo Structure (by ref)") (EventInstigator :type "Controller Object Reference"))
  (returns (ReturnValue :type "Float (double-precision)"))
  (bind _returnvalue (`parent.ModifyDamage` DamageAmount DamageInfo EventInstigator))
  (return (* _returnvalue 1.5)))

(fn `ModifyOutgoingDamage`
  (params (Receiver :type "Actor Object Reference") (DamageType :type "EMordhauDamageType Enum" :default "Generic") (HitInfo :type "HitResult Structure (by ref)") (Agent :type "Actor Object Reference") (InDamage :type "Float (double-precision)"))
  (returns (OutDamage :type "Float (double-precision)"))
  (locals (Multiplier :type "Float (double-precision)" :default 1.0))
  (cast `/Game/Mordhau/Blueprints/GameModes/Horde/BP_HordePlayerController` (`self.GetControllerIncludingVehicle`))
  (`|ExecutionSequence`
    (:`then_0`
      (cast `/Game/Mordhau/Blueprints/Equipment/Ranged/BP_Crossbow` (`self.RightHandEquipment`)
        (:`then`
          (set `local.Multiplier` 1.1))
        (:`CastFailed`
          (cast `/Game/Mordhau/Blueprints/Equipment/Ranged/BP_Bow` (`self.LeftHandEquipment`))
          (set `local.Multiplier` 1.1))))
    (:`then_1`
      (return (* InDamage (`local.Multiplier`))))))

(fn `SaveEquipmentToPlayerState`
  (bind _equipment (`self.Equipment`))
  (bind _asbp_horde_player_controller (cast `/Game/Mordhau/Blueprints/GameModes/Horde/BP_HordePlayerController` (`self.GetControllerIncludingVehicle`)))
  (bind _asbp_horde_player_state (cast `/Game/Mordhau/Blueprints/GameModes/Horde/BP_HordePlayerState` (`Controller.PlayerState` _asbp_horde_player_controller)))
  (bind _lastequipment (`/Game/Mordhau/Blueprints/GameModes/Horde/BP_HordePlayerState.LastEquipment` _asbp_horde_player_state))
  (`KismetArrayLibrary.Array_Clear` _lastequipment)
  (bind _lastequipmentammo (`/Game/Mordhau/Blueprints/GameModes/Horde/BP_HordePlayerState.LastEquipmentAmmo` _asbp_horde_player_state))
  (`KismetArrayLibrary.Array_Clear` _lastequipmentammo)
  (for (_array_element _array_index) _equipment
    (`/Engine/EditorBlueprintResources/StandardMacros.IsValid` _array_element
      (:`Is Valid`
        (if (== (- (`KismetArrayLibrary.Array_Length` _equipment) 1) _array_index)
          (`KismetArrayLibrary.Array_Add` _lastequipment :!label _label)
          (`KismetArrayLibrary.Array_Add` _lastequipmentammo)
          (else
            (`KismetArrayLibrary.Array_Add` _lastequipment (`GameplayStatics.GetObjectClass` _array_element))
            (`KismetArrayLibrary.Array_Add` _lastequipmentammo (`MordhauEquipment.GetAmmo` _array_element)))))
      (:`Is Not Valid`
        (goto _label)))))

(fn `UserConstructionScript`
  (`parent.UserConstructionScript`))